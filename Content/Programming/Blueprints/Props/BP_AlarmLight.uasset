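; BP_AlarmLight is an alarm light prop with two spotlights that spin while the alarm is active.
; SetLight stores the active state and shows or hides both spotlights, with BeginPlay applying the StartActive setting.
; While active, Tick accumulates an angle from RotationSpeed and delta time and applies it as relative roll on the LightRotator component.
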(event `self.ReceiveBeginPlay`
  (`self.Set Light` (`self.StartActive`)))

(event `self.ReceiveTick`
  (params (DeltaSeconds :type "Float (single-precision)"))
  ;[1 1 1] Set new light angle
  (if (`self.IsActive`)
    (bind _output_get (set `self.angle` (+ (* DeltaSeconds (`self.RotationSpeed`)) (`self.angle`))))
    ;[1 1 1] Rotate the light
    (`SceneComponent.K2_SetRelativeRotation` (`self.LightRotator`) (`KismetMathLibrary.MakeRotator` _output_get) false false)))

(fn `Set Light`
  (params (Active :type Boolean))
  (bind _output_get (set `self.IsActive` Active))
  (if _output_get
    ;[1 1 1] Enable/Disable lights
    (`SceneComponent.SetVisibility` (`self.SpotLight`) true false)
    (`SceneComponent.SetVisibility` (`self.SpotLight1`) true false)
    (else
      (`SceneComponent.SetVisibility` (`self.SpotLight1`) false false)
      (`SceneComponent.SetVisibility` (`self.SpotLight`) false false))))

(fn `UserConstructionScript`)