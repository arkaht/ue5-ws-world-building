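; Sliding double sci-fi door prop that opens from a box trigger overlap.
; Unique doors open for any overlapping actor, while others must be unlocked and require a BP_Player with DoorAccess.
; A timeline slides both panels, with a sound played only when the left panel starts at a set position.
; Leaving the trigger reverses the timeline, as does CallCloseDoor on non-Unique doors.
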(event `self.Box.OnComponentBeginOverlap`
  (params (OverlappedComponent :type "PrimitiveComponent Object Reference") (OtherActor :type "Actor Object Reference") (OtherComp :type "PrimitiveComponent Object Reference") (OtherBodyIndex :type Integer) (bFromSweep :type Boolean) (SweepResult :type "HitResult Structure (by ref)"))
  (if (`self.Unique`)
    (if (== (.y (.location (`SceneComponent.GetRelativeTransform` (`self.LeftDoor`)))) 200.0) :!label _label
      (`GameplayStatics.SpawnSoundAtLocation` "/Game/Design/Sounds/PressureChamber/MS_Door_SciFi.MS_Door_SciFi" (`SceneComponent.K2_GetComponentLocation` (`self.LeftFrame`)) (struct) 1.0 1.0 0.0 "/Game/Design/Sounds/BasicAttenuation.BasicAttenuation" "/Game/Design/Sounds/BasicConcurrency.BasicConcurrency")
      (bind (_direction _left _right) (`Timeline|Open/Close Door` :!label _label_2)
        (:`Update`
          (`SceneComponent.K2_SetRelativeTransform` (`self.LeftDoor`) (`KismetMathLibrary.MakeTransform` _left) false false)
          (`SceneComponent.K2_SetRelativeTransform` (`self.RightDoor`) (`KismetMathLibrary.MakeTransform` _right (struct :`Yaw` 180.0)) false false)))
      (else
        (goto _label_2)))
    (elif (not (`self.IsLocked`))
      (bind _asbp_player (cast `/Game/Programming/Blueprints/Core/BP_Player` OtherActor))
      (if (`/Game/Programming/Blueprints/Core/BP_Player.DoorAccess` _asbp_player)
        (goto _label)))))

(event `self.Box.OnComponentEndOverlap`
  (params (OverlappedComponent :type "PrimitiveComponent Object Reference") (OtherActor :type "Actor Object Reference") (OtherComp :type "PrimitiveComponent Object Reference") (OtherBodyIndex :type Integer))
  (goto _label_2 :!via `Reverse`))

(event `CallCloseDoor`
  (if (not (`self.Unique`))
    (goto _label_2 :!via `Reverse`)))

(fn `UserConstructionScript`)