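; BP_LockerModule is a lock box prop that pulses red while its UnlockComportement flag is unset.
; Each Tick, it drives the "controller" vector parameter on the lock box mesh's material slot 1 between black and red with a time-based sine wave.
; The dynamic material instance is requested every frame rather than cached, and nothing here resets the color once the flag is set.
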(event `self.ReceiveTick`
  (params (DeltaSeconds :type "Float (single-precision)"))
  (bind _sm_lockbox_props (`self.SM_LOCKBOX_PROPS`))
  (if (not (`self.UnlockComportement`))
    (bind _returnvalue (`PrimitiveComponent.CreateDynamicMaterialInstance` _sm_lockbox_props 1 (`PrimitiveComponent.GetMaterial` _sm_lockbox_props 1) "None"))
    (`MaterialInstanceDynamic.SetVectorParameterValue` _returnvalue "controller" (`KismetMathLibrary.LinearColorLerp` (struct :`A` 1.0) (struct :`R` 1.0 :`A` 1.0) (/ (+ (`KismetMathLibrary.Sin` (* (`GameplayStatics.GetTimeSeconds`) 10.0)) 1.0) 2.0)))))

(fn `UserConstructionScript`)