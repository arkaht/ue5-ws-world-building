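; BP_NarratorInteraction is an interactable narrator object that steps the player through the start pop-up texts of the opening scenario.
; On each interaction during the player's BeginState, it increments a counter, advances the popup on the player's InGameWidget and plays a beep.
; Once the texts run out, the next interaction hides the popup, clears BeginState and grants the player door access.
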(event `self.BP_InteractionComponent.On Interact`
  (params (`Player Controller` :type "/Game/Programming/Blueprints/Core/BP_PlayerController Object Reference"))
  (bind _returnvalue (`self.K2_GetActorLocation`))
  (bind _returnvalue_2 (+ (`self.popUpCounter`) 1))
  (bind _asbp_player (cast `/Game/Programming/Blueprints/Core/BP_Player` (`GameplayStatics.GetPlayerCharacter` 0)))
  (if (`/Game/Programming/Blueprints/Core/BP_Player.BeginState` _asbp_player)
    (bind _ingamewidget (`/Game/Programming/Blueprints/Core/BP_Player.InGameWidget` _asbp_player))
    (if (> _returnvalue_2 (`KismetArrayLibrary.Array_Length` (`/Game/Programming/Blueprints/UI/BP_InGame.PopupTexts` _ingamewidget)))
      (`/Game/Programming/Blueprints/UI/BP_InGame.Hide Start Popup` _ingamewidget)
      (set `/Game/Programming/Blueprints/Core/BP_Player.BeginState` false _asbp_player)
      (set `/Game/Programming/Blueprints/Core/BP_Player.DoorAccess` true _asbp_player)
      (`GameplayStatics.PlaySoundAtLocation` "/Game/Design/Sounds/Bips/BeepA.BeepA" _returnvalue (struct) 0.4 1.0 0.0 null null null null)
      (else
        (set `self.popUpCounter` _returnvalue_2)
        (`/Game/Programming/Blueprints/UI/BP_InGame.Set Next Start Popup Text` _ingamewidget)
        (`GameplayStatics.PlaySoundAtLocation` "/Game/Design/Sounds/Bips/BeepA.BeepA" _returnvalue (struct) 0.4 1.0 0.0 null null null null)))))

(fn `UserConstructionScript`)