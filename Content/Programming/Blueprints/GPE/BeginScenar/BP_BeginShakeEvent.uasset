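; BP_BeginShakeEvent is an actor that plays recurring camera shake and Niagara bursts while the player's BeginState flag is set.
; Tick reads that flag from BP_Player and accumulates a timer, then starts CameraShakeSource and resets Niagara on reaching a random threshold.
; The threshold is re-rolled every frame, biasing intervals toward its minimum.
; Niagara is deactivated on non-firing ticks, so each activation is brief.
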(event `self.ReceiveTick`
  (params (DeltaSeconds :type "Float (single-precision)"))
  (bind _niagara (`self.Niagara`))
  (bind _returnvalue (+ (`self.Timer`) (`GameplayStatics.GetWorldDeltaSeconds`)))
  (bind _asbp_player (cast `/Game/Programming/Blueprints/Core/BP_Player` (`GameplayStatics.GetPlayerCharacter` 0)))
  (if (`/Game/Programming/Blueprints/Core/BP_Player.BeginState` _asbp_player)
    (if (>= _returnvalue (`KismetMathLibrary.RandomFloatInRange` 3.0 8.0))
      (set `self.Timer` 0.0)
      (`CameraShakeSourceComponent.Start` (`self.CameraShakeSource`))
      (`ActorComponent.Activate` _niagara true)
      (else
        (set `self.Timer` _returnvalue)
        (`ActorComponent.Deactivate` _niagara)))))

(fn `UserConstructionScript`)