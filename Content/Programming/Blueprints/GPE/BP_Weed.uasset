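; BP_Weed is an interactable that gives a temporary screen effect when the player uses it.
; On BeginPlay it caches the first PostProcessVolume tagged PP_Weed; interacting enables that volume, then disables it after Duration.
; CanInteract blocks use while the effect is active or the player holds a grabbed actor.
; DisplayColor only creates a dynamic material instance, as its color-setting nodes never run.
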(event `self.ReceiveBeginPlay`
  (bind _outactors (`GameplayStatics.GetAllActorsWithTag` "PP_Weed"))
  (bind _aspost_process_volume (cast `PostProcessVolume` (`|GetArrayItem` _outactors)))
  (set `self.PostProcess` _aspost_process_volume))

(event `self.BP_InteractionComponent.On Interact`
  (params (`Player Controller` :type "/Game/Programming/Blueprints/Core/BP_PlayerController Object Reference"))
  (bind _postprocess (`self.PostProcess`))
  (`/Engine/EditorBlueprintResources/StandardMacros.IsValid` (`/Game/Programming/Blueprints/Core/BP_PlayerController.BP Player` `Player Controller`)
    (:`Is Valid`
      (set `self.Active` true)
      (set `PostProcessVolume.bEnabled` true _postprocess)
      (`KismetSystemLibrary.Delay` (`self.Duration`))
      (set `PostProcessVolume.bEnabled` false _postprocess)
      (set `self.Active` false))))

(fn `Can Interact`
  (params (`Player Controller` :type "/Game/Programming/Blueprints/Core/BP_PlayerController Object Reference"))
  (returns (`Can Interact` :type Boolean))
  (return (and (not (`KismetSystemLibrary.IsValid` (`/Game/Programming/Blueprints/Core/BP_Player.GrabbedActor` (`/Game/Programming/Blueprints/Core/BP_PlayerController.BP Player` `Player Controller`)))) (not (`self.Active`)))))

(fn `DisplayColor`
  (bind _returnvalue (`PrimitiveComponent.CreateDynamicMaterialInstance` (`self.StaticMesh`) 0 null "None"))
  (if (not false)
    _))

(fn `UserConstructionScript`)