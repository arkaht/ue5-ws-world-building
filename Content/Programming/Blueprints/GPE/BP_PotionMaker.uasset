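; Potion-mixing minigame cauldron where the player pours grabbed ingredients to match a randomly chosen color, spawning a trophy on success.
; BeginPlay shuffles ingredient placements, picks the target color and registers with the room trigger.
; Interacting animates the bottle pour via timelines, mixes primary colors through an enum lookup, parks the ingredient and checks the result.
; Liquid material and Niagara bubbles lerp to each new color, or back to default on reset.
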(event `self.ReceiveBeginPlay`
  (bind _resetbutton (`self.ResetButton`))
  (`self.InitMiniGame`)
  (`/Engine/EditorBlueprintResources/StandardMacros.IsValid` _resetbutton
    (:`Is Valid`
      (add `/Game/Programming/Blueprints/GPE/BP_ResetPotionMaker.On Reset` _resetbutton (delegate `ResetColor`)))))

(event `ResetColor`
  ;[0 1 1 0.33] Reset
  (bind _returnvalue (`PrimitiveComponent.CreateDynamicMaterialInstance` (`self.Liquid`) 0 null "None"))
  (bind _returnvalue_2 (`MaterialInstanceDynamic.K2_GetVectorParameterValue` _returnvalue "Base Color"))
  (bind _output_get (set `self.CurrentColor` "NewEnumerator0"))
  (bind _linearcolor (`self.ConvertEnumToLinearColor` _output_get))
  (set `self.FinalColor` _linearcolor)
  (bind (_direction _newtrack_0) (`Timeline|Timeline_ResetColor` :!via `PlayFromStart`)
    (:`Update`
      (bind _returnvalue_3 (`KismetMathLibrary.LinearColorLerp` _returnvalue_2 (`self.FinalColor`) _newtrack_0))
      (`MaterialInstanceDynamic.SetVectorParameterValue` _returnvalue "Base Color" _returnvalue_3)
      (`FXSystemComponent.SetColorParameter` (`self.NS_Bubbles`) "Color" _returnvalue_3)
      (`FXSystemComponent.SetColorParameter` (`self.NS_Bubbles1`) "Color" _returnvalue_3))
    (:`Finished`
      (`Controller.SetIgnoreMoveInput` (`GameplayStatics.GetPlayerController` 0) false))))

(event `self.BP_InteractionComponent.On Interact`
  (params (`Player Controller` :type "/Game/Programming/Blueprints/Core/BP_PlayerController Object Reference"))
  ;[0 1 0 0.33] Get Ingredient
  (set `self.Putting` true)
  (`Controller.SetIgnoreMoveInput` `Player Controller` true)
  (bind _asbp_ingredient_interactable (cast `/Game/Programming/Blueprints/GPE/BP_Ingredient_Interactable` (`/Game/Programming/Blueprints/Core/BP_Player.GrabbedActor` (`/Game/Programming/Blueprints/Core/BP_PlayerController.BP Player` `Player Controller`))))
  (set `self.Pocket Location` (`self.K2_GetActorLocation` _asbp_ingredient_interactable))
  (`self.K2_SetActorLocation` _asbp_ingredient_interactable (+ (`SceneComponent.K2_GetComponentLocation` (`self.Liquid`)) (`self.Bottle Position`)) false false)
  ;[0 0.5 0 0.33] Turn Bottle
  (bind (_direction _newtrack_0) (`Timeline|Timeline_Turn_Bottle` :!label _label)
    (:`Update`
      (`self.K2_SetActorRotation` _asbp_ingredient_interactable (`KismetMathLibrary.MakeRotator` 0.0 (`KismetMathLibrary.Lerp` 0.0 -90.0 (`CurveFloat.GetFloatValue` (`self.Float Curve`) _newtrack_0)) -90.0) false))
    (:`Finished`
      (if (not (`self.Finish`))
        ;[1 1 1] Switch Color
        (bind _returnvalue (`PrimitiveComponent.CreateDynamicMaterialInstance` (`self.Liquid`) 0 null "None"))
        (bind _returnvalue_2 (`MaterialInstanceDynamic.K2_GetVectorParameterValue` _returnvalue "Base Color"))
        ;;[1 1 1] Change color value
        (bind _newcolor (`self.ChangeMaterialColor` (`self.CurrentColor`) (`/Game/Programming/Blueprints/GPE/BP_Ingredient_Interactable.PrimarColor` _asbp_ingredient_interactable)))
        (bind _output_get (set `self.CurrentColor` _newcolor))
        (bind _linearcolor (`self.ConvertEnumToLinearColor` _output_get))
        (set `self.FinalColor` _linearcolor)
        ;;[1 1 1] Animation Switch Color
        (bind (_direction_2 _newtrack_0_2) (`Timeline|Timeline_Change_Color` :!via `PlayFromStart`)
          (:`Update`
            (bind _returnvalue_3 (`KismetMathLibrary.LinearColorLerp` _returnvalue_2 (`self.FinalColor`) _newtrack_0_2))
            (`MaterialInstanceDynamic.SetVectorParameterValue` _returnvalue "Base Color" _returnvalue_3)
            (`FXSystemComponent.SetColorParameter` (`self.NS_Bubbles`) "Color" _returnvalue_3)
            (`FXSystemComponent.SetColorParameter` (`self.NS_Bubbles1`) "Color" _returnvalue_3))
          (:`Finished`
            (set `self.Finish` true)
            (goto _label :!via `ReverseFromEnd`)))
        (else
          ;[1 0 0 0.33] End Action
          (`self.K2_SetActorLocationAndRotation` :`self` _asbp_ingredient_interactable :`NewLocation` (`self.Pocket Location`))
          (set `self.Finish` false)
          (set `self.Putting` false)
          (`self.PutIngredientInPositions` _asbp_ingredient_interactable)
          (`self.VerifyResult`)
          (`Controller.SetIgnoreMoveInput` (`GameplayStatics.GetPlayerController` 0) false))))))

(fn `Can Interact`
  (params (`Player Controller` :type "/Game/Programming/Blueprints/Core/BP_PlayerController Object Reference"))
  (returns (`Can Interact` :type Boolean))
  (return (and (`KismetSystemLibrary.IsValid` (`/Game/Programming/Blueprints/Core/BP_Player.GrabbedActor` (`/Game/Programming/Blueprints/Core/BP_PlayerController.BP Player` `Player Controller`))) (not (`self.Putting`)))))

(fn `ChangeMaterialColor`
  (params (CurrentColor :type "/Game/Programming/Enums/Enum_Primary_Color Enum" :default "NewEnumerator0") (AddedColor :type "/Game/Programming/Enums/Enum_Primary_Color Enum" :default "NewEnumerator0"))
  (returns (NewColor :type "/Game/Programming/Enums/Enum_Primary_Color Enum"))
  (bind _returnvalue (`|EnumEquality` AddedColor "NewEnumerator3"))
  (bind _returnvalue_2 (`|EnumEquality` AddedColor "NewEnumerator1"))
  (bind _returnvalue_3 (`|EnumEquality` AddedColor "NewEnumerator2"))
  (switch `/Game/Programming/Enums/Enum_Primary_Color` CurrentColor
    (:`NewEnumerator0`
      (return AddedColor))
    (:`NewEnumerator1`
      ;[1 1 1] Red
      (if _returnvalue_2
        (return "NewEnumerator1")
        (elif _returnvalue_3
          (return "NewEnumerator4")
          (elif _returnvalue
            (return "NewEnumerator6")))))
    (:`NewEnumerator2`
      ;[1 1 1] Blue
      (if _returnvalue_2
        (return "NewEnumerator4")
        (elif _returnvalue_3
          (return "NewEnumerator2")
          (elif _returnvalue
            (return "NewEnumerator5")))))
    (:`NewEnumerator3`
      ;[1 1 1] Yellow
      (if _returnvalue_2
        (return "NewEnumerator6")
        (elif _returnvalue_3
          (return "NewEnumerator5")
          (elif _returnvalue
            (return "NewEnumerator3")))))
    (:`NewEnumerator4`
      ;[1 1 1] Purple
      (if _returnvalue_2
        (return "NewEnumerator4")
        (elif _returnvalue_3
          (return "NewEnumerator4")
          (elif _returnvalue
            (return "NewEnumerator7")))))
    (:`NewEnumerator5`
      ;[1 1 1] Green
      (if _returnvalue_2
        (return "NewEnumerator7")
        (elif _returnvalue_3
          (return "NewEnumerator5")
          (elif _returnvalue
            (return "NewEnumerator5")))))
    (:`NewEnumerator6`
      ;[1 1 1] Orange
      (if _returnvalue_2
        (return "NewEnumerator6")
        (elif _returnvalue_3
          (return "NewEnumerator7")
          (elif _returnvalue
            (return "NewEnumerator6")))))
    (:`NewEnumerator7`
      (return "NewEnumerator7"))))

(fn `ConvertEnumToLinearColor`
  (params (`Enum Color` :type "/Game/Programming/Enums/Enum_Primary_Color Enum" :default "NewEnumerator0"))
  (returns (LinearColor :type "LinearColor Structure"))
  (switch `/Game/Programming/Enums/Enum_Primary_Color` `Enum Color`
    (:`NewEnumerator0`
      (return (struct :`G` 1.0 :`B` 1.0 :`A` 1.0)))
    (:`NewEnumerator1`
      (return (struct :`R` 1.0 :`A` 1.0)))
    (:`NewEnumerator2`
      (return (struct :`B` 1.0 :`A` 1.0)))
    (:`NewEnumerator3`
      (return (struct :`R` 1.0 :`G` 1.0 :`A` 1.0)))
    (:`NewEnumerator4`
      (return (struct :`R` 0.5 :`B` 1.0 :`A` 1.0)))
    (:`NewEnumerator5`
      (return (struct :`G` 1.0 :`A` 1.0)))
    (:`NewEnumerator6`
      (return (struct :`R` 1.0 :`G` 0.5 :`A` 1.0)))
    (:`NewEnumerator7`
      (return (struct :`A` 1.0)))))

(fn `InitMiniGame`
  (locals (RandomValue :type Integer) (AllColor :type "Array of /Game/Programming/Enums/Enum_Primary_Color Enum") (IngredientsTransforms :type "Array of Transform Structure"))
  (bind _positionafteruse2 (`self.PositionAfterUse2`))
  (bind _transformafterusing (`self.TransformAfterUsing`))
  (bind _positionafteruse (`self.PositionAfterUse`))
  (bind _positionafteruse1 (`self.PositionAfterUse1`))
  (bind _ingredients (`self.Ingredients`))
  (`KismetArrayLibrary.Array_Add` _transformafterusing (`SceneComponent.K2_GetComponentToWorld` _positionafteruse))
  (`ActorComponent.K2_DestroyComponent` _positionafteruse)
  (`KismetArrayLibrary.Array_Add` _transformafterusing (`SceneComponent.K2_GetComponentToWorld` _positionafteruse1))
  (`ActorComponent.K2_DestroyComponent` _positionafteruse1)
  (`KismetArrayLibrary.Array_Add` _transformafterusing (`SceneComponent.K2_GetComponentToWorld` _positionafteruse2))
  (`ActorComponent.K2_DestroyComponent` _positionafteruse2)
  ;[1 1 1] Take locations of all Ingredients
  (if (`KismetArrayLibrary.Array_IsNotEmpty` _ingredients)
    (for _array_element _ingredients
      (`KismetArrayLibrary.Array_Add` (`local.IngredientsTransforms`) (`self.GetTransform` _array_element)))
    ;[1 1 1] Random Location
    (for _array_element_2 (`self.Ingredients`)
      (bind _output_get (set `local.RandomValue` (`KismetMathLibrary.RandomIntegerInRange` 0 (- (`KismetArrayLibrary.Array_Length` (`local.IngredientsTransforms`)) 1))))
      (`self.K2_SetActorTransform` _array_element_2 (`|GetArrayItem` (`local.IngredientsTransforms`) _output_get) false false)
      (`KismetArrayLibrary.Array_Remove` (`local.IngredientsTransforms`) (`local.RandomValue`)))
    ;[1 1 1] Define Result Color
    (bind _output_get_2 (set `local.RandomValue` (`KismetMathLibrary.RandomIntegerInRange` 0 (- (`KismetArrayLibrary.Array_Length` (`local.AllColor`)) 1))))
    (bind _output_get_3 (set `self.ColorResult` (`|GetArrayItem` (`local.AllColor`) _output_get_2)))
    (set `/Game/Programming/Blueprints/Objects/BP_RulesTrigger.GPE_Chaudron` self (`self.RoomTirgger`))))

(fn `PutIngredientInPositions`
  (params (Object :type "/Game/Programming/Blueprints/GPE/BP_Ingredient_Interactable Object Reference"))
  (locals (SaveIndex :type Integer))
  (bind _returnvalue (`KismetArrayLibrary.Array_Find` (`self.StockIngredients`) Object))
  (bind (_output_location _output_rotation) (`KismetMathLibrary.BreakTransform` (`|GetArrayItem` (`self.TransformAfterUsing`) (`local.SaveIndex`))))
  ;[1 1 1] Detach Objeft from Player
  (bind _asbp_player_controller (cast `/Game/Programming/Blueprints/Core/BP_PlayerController` (`GameplayStatics.GetPlayerController` 0)))
  (bind _bp_player (`/Game/Programming/Blueprints/Core/BP_PlayerController.BP Player` _asbp_player_controller))
  (set `/Game/Programming/Blueprints/Core/BP_Player.IsGrabbingObject?` false _bp_player)
  (`/Game/Programming/Blueprints/Core/BP_Player.DetachObjectFromSelf` _bp_player Object)
  (set `/Game/Programming/Blueprints/Core/BP_Player.GrabbedActor` null _bp_player)
  ;[1 1 1] Enable overlap from Object
  (set `PrimitiveComponent.bGenerateOverlapEvents` true (`/Game/Programming/Blueprints/GPE/BP_Ingredient_Interactable.Sphere` Object))
  (set `local.SaveIndex` _returnvalue)
  (if (== _returnvalue -1)
    (bind _returnvalue_2 (`KismetArrayLibrary.Array_Add` (`self.StockIngredients`) Object))
    (bind (_output_location_2 _output_rotation_2) (`KismetMathLibrary.BreakTransform` (`|GetArrayItem` (`self.TransformAfterUsing`) _returnvalue_2)))
    (`self.K2_SetActorTransform` Object (`KismetMathLibrary.MakeTransform` _output_location_2 _output_rotation_2) false false)
    (else
      ;[1 1 1] Exit element
      (`self.K2_SetActorTransform` Object (`KismetMathLibrary.MakeTransform` _output_location _output_rotation) false false))))

(fn `UserConstructionScript`
  (bind _returnvalue (`PrimitiveComponent.CreateDynamicMaterialInstance` (`self.Liquid`) 0 null "None"))
  (bind _linearcolor (`self.ConvertEnumToLinearColor` "NewEnumerator0"))
  (`MaterialInstanceDynamic.SetVectorParameterValue` _returnvalue "Base Color" _linearcolor)
  (`FXSystemComponent.SetColorParameter` (`self.NS_Bubbles`) "Color" _linearcolor)
  (`FXSystemComponent.SetColorParameter` (`self.NS_Bubbles1`) "Color" _linearcolor))

(fn `VerifyResult`
  (bind _randomobjectspaner (`self.RandomObjectSpaner`))
  (if (`|EnumEquality` (`self.ColorResult`) (`self.CurrentColor`))
    ;[1 1 1] Spawner Trophy
    (`/Engine/EditorBlueprintResources/StandardMacros.IsValid` _randomobjectspaner
      (:`Is Valid`
        (`/Game/Programming/Blueprints/Objects/BP_RandomOjectSpawner.Spawn Trophy` _randomobjectspaner 4)
        (`GameplayStatics.PlaySound2D` "/Game/Design/Sounds/Others/YouWin.YouWin" 1.0 1.0 0.0 null null)))))