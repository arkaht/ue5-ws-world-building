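; BP_ColorSequencer runs a color-sequence puzzle, checking entered color IDs against a random target generated at BeginPlay.
; RegisterInput stores each input, tracks the highest color ID for the random range and assigns the input its color material.
; AddSequenceInput advances on a match or clears progress on a mistake or overflow, returning the result.
; Completion only prints "WIN!", and the generated sequence is also printed.
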(event `self.ReceiveBeginPlay`
  (`self.Generate Sequence` (`self.Sequence Length`)))

(fn `Add Sequence Input`
  (params (ID :type Integer))
  (returns (`Is Correct` :type Boolean))
  (bind _current_sequence (`self.Current Sequence`))
  (bind _sequence (`self.Sequence`))
  (bind _returnvalue (`KismetArrayLibrary.Array_Length` _sequence))
  (bind _returnvalue_2 (`KismetArrayLibrary.Array_Length` _current_sequence))
  (if (<= (+ _returnvalue_2 1) _returnvalue)
    (if (== ID (`|GetArrayItem` _sequence _returnvalue_2))
      (`KismetArrayLibrary.Array_Add` _current_sequence ID)
      (if (== _returnvalue_2 _returnvalue)
        (`KismetSystemLibrary.PrintString` "WIN!"))
      (return true)
      (else
        _)))
  ;[1 1 1 0.33] Reset Current Sequence
  (`KismetArrayLibrary.Array_Clear` _current_sequence)
  (return false))

(fn `Generate Sequence`
  (params (Length :type Integer))
  (bind _sequence (`self.Sequence`))
  ;[1 1 1 0.33] Clear Sequence
  (`KismetArrayLibrary.Array_Clear` _sequence)
  (for _ (range Length)
    (bind _returnvalue (`KismetArrayLibrary.Array_Add` _sequence (`KismetMathLibrary.RandomIntegerInRange` 0 (`self.Max Color ID`))))
    (`KismetSystemLibrary.PrintString` (`KismetStringLibrary.Conv_IntToString` (`|GetArrayItem` _sequence _returnvalue)))))

(fn `Register Input`
  (params (Input :type "/Game/Programming/Blueprints/GPE/BP_ColorSequence_Input Object Reference"))
  (bind _color_id (`/Game/Programming/Blueprints/GPE/BP_ColorSequence_Input.Color ID` Input))
  (`KismetArrayLibrary.Array_Add` (`self.Inputs`) Input)
  ;[1 1 1 0.33] Set Maximum ID
  (set `self.Max Color ID` (`KismetMathLibrary.Max` (`self.Max Color ID`) _color_id))
  ;[1 1 1 0.33] Update Material
  (`/Game/Programming/Blueprints/GPE/BP_ColorSequence_Input.Set Color Material` Input (`|GetArrayItem` (`self.Colors Materials`) _color_id)))

(fn `UserConstructionScript`)