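; Three-bottle pouring puzzle that spawns a trophy through BP_RandomOjectSpawner when all three quantities match their victory values.
; Six transfer functions, one per source and destination pair, move as much as the source holds or the destination has room for.
; Each transfer refreshes both bottles, then checks for victory.
; Update functions, also run on BeginPlay, show each level by Z-scaling and offsetting its component, hiding it when empty.
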(event `self.ReceiveBeginPlay`
  (`self.UpdateBottle1`)
  (`self.Update Bottle 2`)
  (`self.UpdateBottle3`))

(fn `CheckForVictory`
  (if (and (== (`self.Bottle1Quantity`) (`self.Bottle1Victory`)) (== (`self.Bottle2Quantity`) (`self.Bottle2Victory`)) (== (`self.Bottle3Quantity`) (`self.Bottle3Victory`)))
    (bind _returnvalue (`GameplayStatics.GetActorOfClass` "/Game/Programming/Blueprints/Objects/BP_RandomOjectSpawner.BP_RandomOjectSpawner_C"))
    (`/Game/Programming/Blueprints/Objects/BP_RandomOjectSpawner.Spawn Trophy` _returnvalue 3)))

(fn `TransferFrom1To2`
  (locals (value_transfered :type Integer))
  (set `local.value_transfered` (`KismetMathLibrary.Min` (`self.Bottle1Quantity`) (- (`self.Bottle2Max`) (`self.Bottle2Quantity`))))
  (set `self.Bottle1Quantity` (- (`self.Bottle1Quantity`) (`local.value_transfered`)))
  (set `self.Bottle2Quantity` (+ (`self.Bottle2Quantity`) (`local.value_transfered`)))
  (`self.UpdateBottle1`)
  (`self.Update Bottle 2`)
  (`self.CheckForVictory`))

(fn `TransferFrom1To3`
  (locals (value_transfered :type Integer))
  (set `local.value_transfered` (`KismetMathLibrary.Min` (`self.Bottle1Quantity`) (- (`self.Bottle3Max`) (`self.Bottle3Quantity`))))
  (set `self.Bottle1Quantity` (- (`self.Bottle1Quantity`) (`local.value_transfered`)))
  (set `self.Bottle3Quantity` (+ (`self.Bottle3Quantity`) (`local.value_transfered`)))
  (`self.UpdateBottle1`)
  (`self.UpdateBottle3`)
  (`self.CheckForVictory`))

(fn `TransferFrom2To1`
  (locals (value_transfered :type Integer))
  (set `local.value_transfered` (`KismetMathLibrary.Min` (`self.Bottle2Quantity`) (- (`self.Bottle1Max`) (`self.Bottle1Quantity`))))
  (set `self.Bottle2Quantity` (- (`self.Bottle2Quantity`) (`local.value_transfered`)))
  (set `self.Bottle1Quantity` (+ (`self.Bottle1Quantity`) (`local.value_transfered`)))
  (`self.Update Bottle 2`)
  (`self.UpdateBottle1`)
  (`self.CheckForVictory`))

(fn `TransferFrom2To3`
  (locals (value_transfered :type Integer))
  (set `local.value_transfered` (`KismetMathLibrary.Min` (`self.Bottle2Quantity`) (- (`self.Bottle3Max`) (`self.Bottle3Quantity`))))
  (set `self.Bottle2Quantity` (- (`self.Bottle2Quantity`) (`local.value_transfered`)))
  (set `self.Bottle3Quantity` (+ (`self.Bottle3Quantity`) (`local.value_transfered`)))
  (`self.Update Bottle 2`)
  (`self.UpdateBottle3`)
  (`self.CheckForVictory`))

(fn `TransferFrom3To1`
  (locals (value_transfered :type Integer))
  (set `local.value_transfered` (`KismetMathLibrary.Min` (`self.Bottle3Quantity`) (- (`self.Bottle1Max`) (`self.Bottle1Quantity`))))
  (set `self.Bottle3Quantity` (- (`self.Bottle3Quantity`) (`local.value_transfered`)))
  (set `self.Bottle1Quantity` (+ (`self.Bottle1Quantity`) (`local.value_transfered`)))
  (`self.UpdateBottle3`)
  (`self.UpdateBottle1`)
  (`self.CheckForVictory`))

(fn `TransferFrom3To2`
  (locals (value_transfered :type Integer))
  (set `local.value_transfered` (`KismetMathLibrary.Min` (`self.Bottle3Quantity`) (- (`self.Bottle2Max`) (`self.Bottle2Quantity`))))
  (set `self.Bottle3Quantity` (- (`self.Bottle3Quantity`) (`local.value_transfered`)))
  (set `self.Bottle2Quantity` (+ (`self.Bottle2Quantity`) (`local.value_transfered`)))
  (`self.UpdateBottle3`)
  (`self.Update Bottle 2`)
  (`self.CheckForVictory`))

(fn `Update Bottle 2`
  (bind _bottle2 (`self.Bottle2`))
  (bind _bottle2_2 (`self.Bottle2`))
  (bind (_relativescale3d_x _relativescale3d_y) (`KismetMathLibrary.BreakVector` (`SceneComponent.RelativeScale3D` _bottle2)))
  (bind (_relativelocation_x _relativelocation_y) (`KismetMathLibrary.BreakVector` (`SceneComponent.RelativeLocation` _bottle2_2)))
  (if (== (`self.Bottle2Quantity`) 0)
    (`SceneComponent.SetVisibility` (`self.Bottle2`) false false)
    (else
      (`SceneComponent.SetVisibility` (`self.Bottle2`) true false)
      (`SceneComponent.SetRelativeScale3D` _bottle2 (`KismetMathLibrary.MakeVector` _relativescale3d_x _relativescale3d_y (/ (`self.Bottle2Quantity`) 10)))
      (`SceneComponent.K2_SetRelativeLocation` _bottle2_2 (`KismetMathLibrary.MakeVector` _relativelocation_x _relativelocation_y (* (- 12 (`self.Bottle2Quantity`)) -5.0)) false false))))

(fn `UpdateBottle1`
  (bind _bottle1 (`self.Bottle1`))
  (bind _bottle1_2 (`self.Bottle1`))
  (bind (_relativelocation_x _relativelocation_y) (`KismetMathLibrary.BreakVector` (`SceneComponent.RelativeLocation` _bottle1_2)))
  (bind (_relativescale3d_x _relativescale3d_y) (`KismetMathLibrary.BreakVector` (`SceneComponent.RelativeScale3D` _bottle1)))
  (if (== (`self.Bottle1Quantity`) 0)
    (`SceneComponent.SetVisibility` (`self.Bottle1`) false false)
    (else
      (`SceneComponent.SetVisibility` (`self.Bottle1`) true false)
      (`SceneComponent.SetRelativeScale3D` _bottle1 (`KismetMathLibrary.MakeVector` _relativescale3d_x _relativescale3d_y (/ (`self.Bottle1Quantity`) 10)))
      (`SceneComponent.K2_SetRelativeLocation` _bottle1_2 (`KismetMathLibrary.MakeVector` _relativelocation_x _relativelocation_y (* (- 12 (`self.Bottle1Quantity`)) -5.0)) false false))))

(fn `UpdateBottle3`
  (bind _bottle3 (`self.Bottle3`))
  (bind _bottle3_2 (`self.Bottle3`))
  (bind (_relativescale3d_x _relativescale3d_y) (`KismetMathLibrary.BreakVector` (`SceneComponent.RelativeScale3D` _bottle3)))
  (bind (_relativelocation_x _relativelocation_y) (`KismetMathLibrary.BreakVector` (`SceneComponent.RelativeLocation` _bottle3_2)))
  (if (== (`self.Bottle3Quantity`) 0)
    (`SceneComponent.SetVisibility` (`self.Bottle3`) false false)
    (else
      (`SceneComponent.SetVisibility` (`self.Bottle3`) true false)
      (`SceneComponent.SetRelativeScale3D` _bottle3 (`KismetMathLibrary.MakeVector` _relativescale3d_x _relativescale3d_y (/ (`self.Bottle3Quantity`) 10)))
      (`SceneComponent.K2_SetRelativeLocation` _bottle3_2 (`KismetMathLibrary.MakeVector` _relativelocation_x _relativelocation_y (* (- 12 (`self.Bottle3Quantity`)) -5.0)) false false))))

(fn `UserConstructionScript`)