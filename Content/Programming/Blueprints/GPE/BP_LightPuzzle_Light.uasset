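; A puzzle light actor for a light puzzle, with a point light and a sphere that show whether it is on or off.
; BeginPlay applies the initial Activated state through ChangeLight.
; SwitchLight flips Activated and calls ChangeLight, which sets the point light intensity and swaps the sphere between on and off materials.
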(event `self.ReceiveBeginPlay`
  (`self.ChangeLight` (`self.Activated`)))

(fn `ChangeLight`
  (params (LightActivated :type Boolean))
  (bind _sphere (`self.Sphere`))
  (bind _pointlight (`self.PointLight`))
  (if LightActivated
    (`LightComponent.SetIntensity` _pointlight 10000.0)
    (`PrimitiveComponent.SetMaterial` _sphere 0 (`self.OnMat`))
    (else
      (`LightComponent.SetIntensity` _pointlight 0.0)
      (`PrimitiveComponent.SetMaterial` _sphere 0 (`self.OffMat`)))))

(fn `SwitchLight`
  (bind _output_get (set `self.Activated` (not (`self.Activated`))))
  (`self.ChangeLight` _output_get))

(fn `UserConstructionScript`)