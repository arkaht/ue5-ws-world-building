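; Interactable gameplay entity that cycles the material on its static mesh.
; Each OnInteract event from its BP_InteractionComponent advances CurrentMaterialID through the Materials array, wrapping with modulo, and applies that material to element 0.
; CanInteract always returns true, so it places no condition on interaction.
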(event `self.BP_InteractionComponent.On Interact`
  (params (`Player Controller` :type "/Game/Programming/Blueprints/Core/BP_PlayerController Object Reference"))
  (bind _materials (`self.Materials`))
  ;[1 1 1 0.33] Get Next Index
  (bind _output_get (set `self.Current Material ID` (mod (+ (`self.Current Material ID`) 1) (`KismetArrayLibrary.Array_Length` _materials))))
  ;[1 1 1 0.33] Set Material
  (`PrimitiveComponent.SetMaterial` (`self.StaticMesh`) 0 (`|GetArrayItem` _materials _output_get)))

(fn `Can Interact`
  (params (`Player Controller` :type "/Game/Programming/Blueprints/Core/BP_PlayerController Object Reference"))
  (returns (`Can Interact` :type Boolean))
  (return true))

(fn `UserConstructionScript`)