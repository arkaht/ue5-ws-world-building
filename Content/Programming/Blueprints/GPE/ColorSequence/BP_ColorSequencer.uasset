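; Sequencer for a Simon-style color puzzle that runs data-defined rounds of random color sequences the player must reproduce.
; Registered inputs set the color ID range, and each round generates a sequence with no consecutive repeats.
; Correct entries advance toward the next round, while a wrong one restarts the round with a fresh sequence.
; Dispatchers announce round starts, accepted inputs and final success.
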(fn `Add Sequence Input`
  (params (ID :type Integer))
  (returns (`Is Correct` :type Boolean))
  (bind _current_sequence (`self.Current Sequence`))
  (bind _sequence (`self.Sequence`))
  (bind _returnvalue (`KismetArrayLibrary.Array_Length` _sequence))
  (bind _returnvalue_2 (`KismetArrayLibrary.Array_Length` _current_sequence))
  ;[1 1 1 0.33] Check is in Round
  (if (`KismetArrayLibrary.Array_IsValidIndex` (`/Game/Programming/Blueprints/Data/BP_ColorSequencerData.Rounds` (`self.Data`)) (`self.Current Round ID`))
    (if (<= (+ _returnvalue_2 1) _returnvalue)
      (if (== ID (`|GetArrayItem` _sequence _returnvalue_2))
        (`KismetArrayLibrary.Array_Add` _current_sequence ID)
        (`self.On Input` ID)
        (if (== _returnvalue_2 _returnvalue)
          (`KismetSystemLibrary.PrintString` "WIN!")
          (`self.Next Round`))
        (return true)
        (else
          _)))
    (`self.Start Round`)
    (return false)))

(fn `Generate Sequence`
  (params (Length :type Integer))
  (locals (`Generated ID` :type Integer) (`Last ID` :type Integer :default -1))
  (bind _sequence (`self.Sequence`))
  (bind _generated_id (`local.Generated ID`))
  ;[1 1 1 0.33] Clear Sequence
  (`KismetArrayLibrary.Array_Clear` _sequence)
  (for _ (range Length)
    (set `local.Generated ID` (`KismetMathLibrary.RandomIntegerInRange` 0 (`self.Max Color ID`)) :!label _label)
    (if (== (`local.Last ID`) _generated_id)
      (goto _label)
      (else
        (bind _output_get (set `local.Last ID` _generated_id))
        (`KismetArrayLibrary.Array_Add` _sequence _output_get)))))

(fn `Next Round`
  (bind _result (`/Engine/EditorBlueprintResources/StandardMacros.IncrementInt` (`self.Current Round ID`))
    (:`  `
      (if (< _result (`KismetArrayLibrary.Array_Length` (`/Game/Programming/Blueprints/Data/BP_ColorSequencerData.Rounds` (`self.Data`))))
        (`self.Start Round`)
        (else
          (`self.On Success`))))))

(fn `Register Input`
  (params (Input :type "/Game/Programming/Blueprints/GPE/ColorSequence/BP_ColorSequence_Input Object Reference"))
  (`KismetArrayLibrary.Array_Add` (`self.Inputs`) Input)
  ;[1 1 1 0.33] Set Maximum ID
  (set `self.Max Color ID` (`KismetMathLibrary.Max` (`self.Max Color ID`) (`/Game/Programming/Blueprints/GPE/ColorSequence/BP_ColorSequence_Input.Color ID` Input))))

(fn `Start Round`
  (bind _output (`|GetArrayItem` (`/Game/Programming/Blueprints/Data/BP_ColorSequencerData.Rounds` (`self.Data`)) (`self.Current Round ID`)))
  ;[1 1 1 0.33] Reset Current Sequence
  (`KismetArrayLibrary.Array_Clear` (`self.Current Sequence`))
  ;[1 1 1 0.33] Generate Sequence
  (`self.Generate Sequence` (`.SequenceLength_3_1AB6D4854CF6C0C24B95CF9C5AF8BDAB` (break `/Game/Programming/Structs/S_ColorSequence_Round` _output)))
  (set `self.Is Showing on Screens` true)
  (`self.On Round Start` _output))

(fn `UserConstructionScript`)