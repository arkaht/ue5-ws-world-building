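; BP_ColorSequence_Input is an interactable button that feeds one color into a color-sequence puzzle run by its assigned Sequencer.
; On BeginPlay it registers with the Sequencer, takes its mesh and material by ColorID and its use time from the Sequencer's Data, and logs a warning if none is assigned.
; Interacting sends its ColorID to the Sequencer, and CanInteract blocks use while the Sequencer is showing on screens.
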(event `self.ReceiveBeginPlay`
  (`|ExecutionSequence`
    (:`then_0`
      ;[1 1 1 0.33] Register Input
      (bind _sequencer (`self.Sequencer`)
        (:`then`
          (`/Game/Programming/Blueprints/GPE/ColorSequence/BP_ColorSequencer.Register Input` _sequencer self)
          (`self.Setup Mesh and Material`))
        (:`else`
          (`KismetSystemLibrary.PrintString` "BP_ColorSequence_Input: no Sequencer has been assigned, the Input won't work as intended" true true (struct :`R` 1.0 :`G` 0.083333 :`A` 1.0) 10.0))))
    (:`then_1`
      ;[1 1 1 0.33] Set Custom Use Time
      (set `/Game/Programming/Blueprints/GPE/BP_InteractionComponent.Use Time` (`/Game/Programming/Blueprints/Data/BP_ColorSequencerData.Inputs Use Time` (`/Game/Programming/Blueprints/GPE/ColorSequence/BP_ColorSequencer.Data` (`self.Sequencer`))) (`self.BP_InteractionComponent`)))))

(event `self.BP_InteractionComponent.On Interact`
  (params (`Player Controller` :type "/Game/Programming/Blueprints/Core/BP_PlayerController Object Reference"))
  (`/Game/Programming/Blueprints/GPE/ColorSequence/BP_ColorSequencer.Add Sequence Input` (`self.Sequencer`) (`self.Color ID`)))

(fn `Can Interact`
  (params (`Player Controller` :type "/Game/Programming/Blueprints/Core/BP_PlayerController Object Reference"))
  (returns (`Can Interact` :type Boolean))
  (return (not (`/Game/Programming/Blueprints/GPE/ColorSequence/BP_ColorSequencer.Is Showing on Screens` (`self.Sequencer`)))))

(fn `Setup Mesh and Material`
  (bind _sm_button (`self.SM Button`))
  (bind _color_id (`self.Color ID`))
  (bind _data (`/Game/Programming/Blueprints/GPE/ColorSequence/BP_ColorSequencer.Data` (`self.Sequencer`)))
  (`StaticMeshComponent.SetStaticMesh` _sm_button (`|GetArrayItem` (`/Game/Programming/Blueprints/Data/BP_ColorSequencerData.Meshes` _data) _color_id))
  (`PrimitiveComponent.SetMaterial` _sm_button 0 (`|GetArrayItem` (`/Game/Programming/Blueprints/Data/BP_ColorSequencerData.Materials` _data) _color_id)))

(fn `UserConstructionScript`)