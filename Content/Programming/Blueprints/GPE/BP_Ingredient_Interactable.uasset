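; Interactable ingredient actor that hands itself to the player when used.
; On interact, it checks that the controller's player is valid, disables overlap events on its sphere and calls the player's OnTrophyInteraction.
; DisplayColor toggles the mesh's Base Color between its primary-color tint and SaveColor through a dynamic material instance.
; The construction-script logic that captured SaveColor and applied the tint is disconnected, as is an older non-animated grab path.
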(event `self.BP_InteractionComponent.On Interact`
  (params (`Player Controller` :type "/Game/Programming/Blueprints/Core/BP_PlayerController Object Reference"))
  (bind _bp_player (`/Game/Programming/Blueprints/Core/BP_PlayerController.BP Player` `Player Controller`))
  (`/Engine/EditorBlueprintResources/StandardMacros.IsValid` _bp_player
    (:`Is Valid`
      (set `PrimitiveComponent.bGenerateOverlapEvents` false (`self.Sphere`))
      (`/Game/Programming/Blueprints/Core/BP_Player.OnTrophyInteraction` _bp_player self))))

(fn `DisplayColor`
  (bind _returnvalue (`PrimitiveComponent.CreateDynamicMaterialInstance` (`self.StaticMesh`) 0 null "None"))
  (if (not (`self.On/Off`))
    (set `self.On/Off` true)
    (switch `/Game/Programming/Enums/Enum_Primary_Color` (`self.PrimarColor`)
      (:`NewEnumerator0`
        (`MaterialInstanceDynamic.SetVectorParameterValue` _returnvalue "Base Color" (struct :`G` 1.0 :`B` 1.0 :`A` 1.0)))
      (:`NewEnumerator1`
        (`MaterialInstanceDynamic.SetVectorParameterValue` _returnvalue "Base Color" (struct :`R` 1.0 :`A` 1.0)))
      (:`NewEnumerator2`
        (`MaterialInstanceDynamic.SetVectorParameterValue` _returnvalue "Base Color" (struct :`B` 1.0 :`A` 1.0)))
      (:`NewEnumerator3`
        (`MaterialInstanceDynamic.SetVectorParameterValue` _returnvalue "Base Color" (struct :`R` 1.0 :`G` 1.0 :`A` 1.0))))
    (else
      (set `self.On/Off` false)
      (`MaterialInstanceDynamic.SetVectorParameterValue` _returnvalue "Base Color" (`self.SaveColor`)))))

(fn `UserConstructionScript`)