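; Manager actor for a Spot the Difference puzzle that moves a glass pane once every interactable object is correct.
; On BeginPlay it gathers all BP_STD_Interactable actors in the level and hands each a reference to itself.
; VerifyAllObjects polls each object, and when all pass, it disables their interaction and plays a timeline that drives the pane's world Z position.
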(event `self.ReceiveBeginPlay`
  (`self.ReferenceAllObjects`))

(event `MoveGlassPane`
  (bind _glasspane (`self.GlassPane`))
  (bind (_returnvalue_x _returnvalue_y) (`KismetMathLibrary.BreakVector` (`self.K2_GetActorLocation` _glasspane)))
  (bind (_direction _glassheightmovement) (`Timeline|GlassPaneOut`)
    (:`Update`
      (`self.K2_SetActorLocation` _glasspane (`KismetMathLibrary.MakeVector` _returnvalue_x _returnvalue_y _glassheightmovement) false false))))

(fn `AllObjectsAreVerified`
  (for _array_element (`self.AllInteractablesArray`)
    (set `/Game/Programming/Blueprints/GPE/SpotTheDifference/BP_STD_Interactable.CanBeInteracteedWith` false _array_element))
  (`self.MoveGlassPane`))

(fn `ReferenceAllObjects`
  ;[1 0.3379 0.6043] Get References
  (bind _outactors (`GameplayStatics.GetAllActorsOfClass` "/Game/Programming/Blueprints/GPE/SpotTheDifference/BP_STD_Interactable.BP_STD_Interactable_C"))
  (bind _output_get (set `self.AllInteractablesArray` _outactors))
  ;[0.3977 0.2188 1] Make them get reference
  (for _array_element _output_get
    (`/Game/Programming/Blueprints/GPE/SpotTheDifference/BP_STD_Interactable.ReferenceSTDManager` _array_element self)))

(fn `UserConstructionScript`)

(fn `VerifyAllObjects`
  (locals (FinalResult :type Boolean))
  (set `local.FinalResult` true)
  (for _array_element (`self.AllInteractablesArray`)
    (bind _iscorrect (`/Game/Programming/Blueprints/GPE/SpotTheDifference/BP_STD_Interactable.VerifyIfCorrect` _array_element))
    (if (not _iscorrect)
      (set `local.FinalResult` false)))
  (if (`local.FinalResult`)
    (`self.AllObjectsAreVerified`)))