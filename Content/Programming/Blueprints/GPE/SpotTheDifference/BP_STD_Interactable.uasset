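; Spot-the-difference puzzle object that, on interaction, cycles its position, rotation, material or mesh, according to its InteractionType.
; A cooldown gates input, with timelines animating rotation and a height wiggle on mesh swaps.
; Each change asks the injected STDManager to verify all objects, while VerifyIfCorrect compares state to the solution.
; On BeginPlay, mesh swaps can randomize a mirrored solution with a different start, or a matching decoy.
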(event `self.ReceiveBeginPlay`
  ;[0.2708 0.2708 0.2708] BEGIN PLAY
  (`self.GetReferences`)
  (`self.GenerateRandomSolution`))

(event `self.BP_InteractionComponent.On Interact`
  (params (`Player Controller` :type "/Game/Programming/Blueprints/Core/BP_PlayerController Object Reference"))
  (if (`self.CanBeInteracteedWith`)
    (if (not (`self.isInCooldown`))
      (set `self.isInCooldown` true)
      (switch `/Game/Programming/Enums/ESTDInteractionType` (`self.InteractionType`)
        (:`NewEnumerator2`
          (`self.MoveInteractable`)
          (`/Game/Programming/Blueprints/GPE/SpotTheDifference/BP_STD_Manager.VerifyAllObjects` (`self.STD_Manager`) :!label _label))
        (:`NewEnumerator0`
          (`self.Rotate Interactable`))
        (:`NewEnumerator1`
          (`self.SwitchColorMaterial`)
          (goto _label))
        (:`NewEnumerator3`
          (`self.SwitchStaticMesh`))))))

(event `LaunchCooldown`
  (`KismetSystemLibrary.Delay` 0.7)
  (set `self.isInCooldown` false))

(event `MeshReplacementWiggle`
  (bind _interactablemesh (`self.InteractableMesh`))
  (bind (_returnvalue_x _returnvalue_y) (`KismetMathLibrary.BreakVector` (`SceneComponent.K2_GetComponentScale` _interactablemesh)))
  (bind (_direction _heightwiggle) (`Timeline|MeshWiggleTimeline` :!via `PlayFromStart`)
    (:`Update`
      (`SceneComponent.SetWorldScale3D` _interactablemesh (`KismetMathLibrary.MakeVector` _returnvalue_x _returnvalue_y (* (`self.InteractableStartingHeight`) _heightwiggle))))
    (:`Finished`
      (set `self.isInCooldown` false :!label _label_2)
      (`/Game/Programming/Blueprints/GPE/SpotTheDifference/BP_STD_Manager.VerifyAllObjects` (`self.STD_Manager`)))))

(event `RotationLerp`
  (bind _interactablemesh (`self.InteractableMesh`))
  (bind (_relativerotation_roll _relativerotation_pitch _relativerotation_yaw) (`KismetMathLibrary.BreakRotator` (`SceneComponent.RelativeRotation` (`self.InteractableMesh`))))
  (bind (_relativerotation_roll_2 _relativerotation_pitch_2) (`KismetMathLibrary.BreakRotator` (`SceneComponent.RelativeRotation` _interactablemesh)))
  (set `self.StartingRotation` _relativerotation_yaw)
  (bind (_direction _newtrack_0) (`Timeline|RotationLerpTimeline` :!via `PlayFromStart`)
    (:`Update`
      (`SceneComponent.K2_SetRelativeRotation` _interactablemesh (`KismetMathLibrary.MakeRotator` _relativerotation_roll_2 _relativerotation_pitch_2 (+ (* _newtrack_0 (`self.RotationAmountDegrees`)) (`self.StartingRotation`))) false false))
    (:`Finished`
      (goto _label_2))))

(fn `GenerateRandomSolution`
  (locals (FirstIndex :type Integer) (SecondIndex :type Integer))
  (bind _meshpossibilities (`self.MeshPossibilities`))
  (bind _returnvalue (- (`KismetArrayLibrary.Array_Length` (`self.MeshPossibilities`)) 1))
  (switch `/Game/Programming/Enums/ESTDInteractionType` (`self.InteractionType`)
    (:`NewEnumerator3`
      (if (`self.RandomlyGenerateCorrectMeshSolution`)
        ;[0.3176 0.3319 1] Set the mesh to match
        (bind _output_get (set `local.FirstIndex` (`KismetMathLibrary.RandomIntegerInRange` 0 _returnvalue)))
        (bind _output_get_2 (set `self.ValidMeshIndex` _output_get))
        (`StaticMeshComponent.SetStaticMesh` (`self.MirroredMesh`) (`|GetArrayItem` (`self.MeshPossibilities`) _output_get_2))
        (set `local.SecondIndex` (`KismetMathLibrary.RandomIntegerInRange` 0 _returnvalue))
        ;[0.1183 1 0.2471] Don't start at the correct one
        (if (== (`local.FirstIndex`) (`local.SecondIndex`))
          ;[0.237 0.9402 1] Set the mesh to modify
          (bind _output_get_3 (set `local.SecondIndex` (mod (+ (`local.SecondIndex`) 1) (`KismetArrayLibrary.Array_Length` (`self.MeshPossibilities`)))))
          (bind _output_get_4 (set `self.CurrentMeshIndex` _output_get_3))
          (`StaticMeshComponent.SetStaticMesh` (`self.InteractableMesh`) (`|GetArrayItem` _meshpossibilities _output_get_4))
          (else
            (bind _output_get_5 (set `self.CurrentMeshIndex` (`local.SecondIndex`)))
            (`StaticMeshComponent.SetStaticMesh` (`self.InteractableMesh`) (`|GetArrayItem` _meshpossibilities _output_get_5))))
        (elif (`self.ShouldCreateFakeMesh`)
          (bind _output_get_6 (set `self.CurrentMeshIndex` (`KismetMathLibrary.RandomIntegerInRange` 0 (- (`KismetArrayLibrary.Array_Length` (`self.MeshPossibilities`)) 1))))
          (set `self.ValidMeshIndex` _output_get_6)
          (bind _output (`|GetArrayItem` (`self.MeshPossibilities`) _output_get_6))
          (`StaticMeshComponent.SetStaticMesh` (`self.InteractableMesh`) _output)
          (`StaticMeshComponent.SetStaticMesh` (`self.MirroredMesh`) _output))))))

(fn `GetReferences`
  (bind _movementpositions (`self.MovementPositions`))
  (bind (_returnvalue_x _returnvalue_y _returnvalue_z) (`KismetMathLibrary.BreakVector` (`SceneComponent.K2_GetComponentScale` (`self.InteractableMesh`))))
  (`|ExecutionSequence`
    (:`then_0`
      ;[0.2389 0.6141 1] Create array of possible positions
      (if (`|EnumEquality` (`self.InteractionType`) "NewEnumerator2")
        (set `self.MovementPositions` (`|MakeArray` (`self.MovementPosition_0`) (`self.MovementPosition_1`) (`self.MovementPosition_2`) (`self.MovementPosition_3`)))
        ;[0.9713 0.3431 1] Remove so that only the first X are taken into account (if there should be only 3 positions, don't loop between 4)
        (switch `int` (`self.TotalNumberOfPositions`)
          (:`0`
            ;[1 0.1647 0.1349] Signal error if there isn't enough positions to swap between (0 or 1 total)
            (`KismetSystemLibrary.PrintText` (`|FormatText` "/!\\ WARNING /!\\ \nSTD_Interactable with name \n{ObjectName} \nis set to have Movement interaction, but number of positions is < 2" (`KismetSystemLibrary.GetDisplayName` self)) true true (struct :`R` 1.0 :`B` 0.025391 :`A` 1.0) 50.0 :!label _label))
          (:`1`
            (goto _label))
          (:`2`
            (`KismetArrayLibrary.Array_Remove` _movementpositions 3)
            (`KismetArrayLibrary.Array_Remove` _movementpositions 2))
          (:`3`
            (`KismetArrayLibrary.Array_Remove` _movementpositions 3)))))
    (:`then_1`
      (set `self.InteractableStartingHeight` _returnvalue_z))))

(fn `MoveInteractable`
  ;[0.1697 0.6725 1] Increment value (with modulo)
  (bind _output_get (set `self.CurrentPositionIndex` (mod (+ (`self.CurrentPositionIndex`) 1) (`self.TotalNumberOfPositions`))))
  ;[1 0.9774 0.2282] Set to new position
  (`SceneComponent.K2_SetWorldLocation` (`self.InteractableMesh`) (`SceneComponent.K2_GetComponentLocation` (`|GetArrayItem` (`self.MovementPositions`) _output_get)) false false)
  (`self.VerifyIfCorrect`)
  (`self.LaunchCooldown`))

(fn `ReferenceSTDManager`
  (params (NewParam :type "/Game/Programming/Blueprints/GPE/SpotTheDifference/BP_STD_Manager Object Reference"))
  (set `self.STD_Manager` NewParam))

(fn `Rotate Interactable`
  (`self.RotationLerp`))

(fn `SwitchColorMaterial`
  ;[0.1697 0.6725 1] Increment value (with modulo)
  (bind _output_get (set `self.CurrentMaterialIndex` (mod (+ (`self.CurrentMaterialIndex`) 1) (`KismetArrayLibrary.Array_Length` (`self.MaterialList`)))))
  ;[1 0.9774 0.2282] Set new Material visually
  (`PrimitiveComponent.SetMaterial` (`self.InteractableMesh`) (`self.MaterialIDToChange`) (`|GetArrayItem` (`self.MaterialList`) _output_get))
  (`GameplayStatics.PlaySound2D` "/Game/Design/Sounds/Splashes/MS_Splash.MS_Splash" 1.5 1.0 0.0 null null)
  (`self.VerifyIfCorrect`)
  (`self.LaunchCooldown`))

(fn `SwitchStaticMesh`
  ;[0.1697 0.6725 1] Increment value (with modulo)
  (bind _output_get (set `self.CurrentMeshIndex` (mod (+ (`self.CurrentMeshIndex`) 1) (`KismetArrayLibrary.Array_Length` (`self.MeshPossibilities`)))))
  ;[1 0.9774 0.2282] Set new Mesh visually
  (`StaticMeshComponent.SetStaticMesh` (`self.InteractableMesh`) (`|GetArrayItem` (`self.MeshPossibilities`) _output_get))
  (`self.MeshReplacementWiggle`))

(fn `UserConstructionScript`)

(fn `VerifyIfCorrect`
  (returns (isCorrect :type Boolean))
  (bind (_relativerotation_roll _relativerotation_pitch _relativerotation_yaw) (`KismetMathLibrary.BreakRotator` (`SceneComponent.RelativeRotation` (`self.InteractableMesh`))))
  (switch `/Game/Programming/Enums/ESTDInteractionType` (`self.InteractionType`)
    (:`NewEnumerator2`
      (return (== (`self.CurrentPositionIndex`) (`self.ValidPositionIndex`))))
    (:`NewEnumerator0`
      (return (< (`KismetMathLibrary.Abs` (- (`self.RotationToMatch`) _relativerotation_yaw)) 5.0)) ; Z
    )
    (:`NewEnumerator1`
      (return (== (`self.CurrentMaterialIndex`) (`self.ValidMaterialIndex`))))
    (:`NewEnumerator3`
      (return (== (`self.CurrentMeshIndex`) (`self.ValidMeshIndex`))))))