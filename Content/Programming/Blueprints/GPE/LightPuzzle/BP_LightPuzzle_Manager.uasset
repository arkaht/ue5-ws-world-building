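; BP_LightPuzzle_Manager tracks the light puzzle and rewards a trophy once every light is activated.
; On BeginPlay it caches all BP_LightPuzzle_Light actors in the level.
; CheckVictory, which nothing in this Blueprint calls, scans those lights and stops at the first inactive one.
; If all are active, it finds the BP_RandomOjectSpawner in the level and calls SpawnTrophy with a hard-coded argument.
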(event `self.ReceiveBeginPlay`
  (bind _outactors (`GameplayStatics.GetAllActorsOfClass` "/Game/Programming/Blueprints/GPE/LightPuzzle/BP_LightPuzzle_Light.BP_LightPuzzle_Light_C"))
  (set `self.Lights` _outactors))

(fn `CheckVictory`
  (locals (all_activated :type Boolean))
  (set `local.all_activated` true)
  (for _array_element (`self.Lights`)
    (if (not (`/Game/Programming/Blueprints/GPE/LightPuzzle/BP_LightPuzzle_Light.Activated` _array_element))
      (set `local.all_activated` false)
      (break)))
  (if (`local.all_activated`)
    (bind _returnvalue (`GameplayStatics.GetActorOfClass` "/Game/Programming/Blueprints/Objects/BP_RandomOjectSpawner.BP_RandomOjectSpawner_C"))
    (`/Game/Programming/Blueprints/Objects/BP_RandomOjectSpawner.Spawn Trophy` _returnvalue 2)))

(fn `UserConstructionScript`)