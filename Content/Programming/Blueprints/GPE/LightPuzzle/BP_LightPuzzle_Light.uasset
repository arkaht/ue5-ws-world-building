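; BP_LightPuzzle_Light is a light element for a light puzzle, shown as a sphere that reads as on or off.
; ChangeLight swaps the sphere's material between OnMat and OffMat, and BeginPlay calls it to display the initial Activated state.
; SwitchLight flips Activated and refreshes the material through ChangeLight.
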(event `self.ReceiveBeginPlay`
  (`self.ChangeLight` (`self.Activated`)))

(fn `ChangeLight`
  (params (LightActivated :type Boolean))
  (bind _sphere (`self.Sphere`))
  (if LightActivated
    (`PrimitiveComponent.SetMaterial` _sphere 0 (`self.OnMat`))
    (else
      (`PrimitiveComponent.SetMaterial` _sphere 0 (`self.OffMat`)))))

(fn `SwitchLight`
  (bind _output_get (set `self.Activated` (not (`self.Activated`))))
  (`self.ChangeLight` _output_get))

(fn `UserConstructionScript`)