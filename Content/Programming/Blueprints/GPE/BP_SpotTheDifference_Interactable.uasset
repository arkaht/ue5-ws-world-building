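; Interactable prop for a spot-the-difference puzzle that rotates its mesh each time E is pressed.
; For the Rotation interaction type, each press adds a configured local rotation on the chosen axis, then calls VerifyIfCorrect.
; That check compares the mesh's relative angle to the target within a small tolerance and only prints the result.
; GetReferences runs at BeginPlay but leaves the player character reference empty.
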(event `self.ReceiveBeginPlay`
  ;[0.2708 0.2708 0.2708] BEGIN PLAY
  (`self.GetReferences`))

(event `Key|E`
  (params (Key :type "Key Structure"))
  (bind _rotationamountdegrees (`self.RotationAmountDegrees`))
  (:`Pressed`
    (switch `/Game/Programming/Enums/ESTDInteractionType` (`self.InteractionType`)
      (:`NewEnumerator0`
        ;[1 0.2471 0.4281] Rotate the Interactable by the correct amount on the correct axis
        (`SceneComponent.K2_AddLocalRotation` (`self.InteractableMesh`) (select `ERigControlAxis` (`self.RotationAxis`) :`X` (`KismetMathLibrary.MakeRotator` _rotationamountdegrees) :`Y` (`KismetMathLibrary.MakeRotator` 0.0 _rotationamountdegrees) :`Z` (`KismetMathLibrary.MakeRotator` 0.0 0.0 _rotationamountdegrees) :!type "Rotator Structure") false false)
        (`self.VerifyIfCorrect`)))))

(fn `GetReferences`
  (`|ExecutionSequence`
    (:`then_0`
      (bind _returnvalue (`GameplayStatics.GetActorOfClass` null))
      (set `self.PlayerCharacterReference` null _returnvalue))))

(fn `UserConstructionScript`)

(fn `VerifyIfCorrect`
  (bind _rotationtomatch (`self.RotationToMatch`))
  (bind (_relativerotation_roll _relativerotation_pitch _relativerotation_yaw) (`KismetMathLibrary.BreakRotator` (`SceneComponent.RelativeRotation` (`self.InteractableMesh`))))
  (switch `/Game/Programming/Enums/ESTDInteractionType` (`self.InteractionType`)
    (:`NewEnumerator0`
      ;[1 0.8299 0.2633] Get the interactable rotation & the rotation to match
      (switch `ERigControlAxis` (`self.RotationAxis`)
        (:`X`
          ;[1 0.07239 0.06244] print this shit
          (`KismetSystemLibrary.PrintText` (`|FormatText` "Rotation to Match : {Target} \nCurrent Rotation : {Current} \nIs Validated : {Bool}" _rotationtomatch _relativerotation_roll (< (`KismetMathLibrary.Abs` (- _rotationtomatch _relativerotation_roll)) 5.0))))
        (:`Y`
          (`KismetSystemLibrary.PrintText` (`|FormatText` "Rotation to Match : {Target} \nCurrent Rotation : {Current} \nIs Validated : {Bool}" _rotationtomatch _relativerotation_pitch (< (`KismetMathLibrary.Abs` (- _rotationtomatch _relativerotation_pitch)) 5.0))))
        (:`Z`
          (`KismetSystemLibrary.PrintText` (`|FormatText` "Rotation to Match : {Target} \nCurrent Rotation : {Current} \nIs Validated : {Bool}" _rotationtomatch _relativerotation_yaw (< (`KismetMathLibrary.Abs` (- _rotationtomatch _relativerotation_yaw)) 5.0))))))))