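; Interactive jukebox prop that plays playlists of sounds from its Data variable and is paused on BeginPlay.
; Interacting while paused resumes playback; otherwise it skips to the next playlist, pausing again when the selection wraps to the first one.
; When a sound finishes, the audio component plays the next one in the current playlist, looping back at the end.
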(event `self.ReceiveBeginPlay`
  (`self.Next Playlist`)
  (`AudioComponent.SetPaused` (`self.Audio`) true))

(event `self.BP_InteractionComponent.On Interact`
  (params (`Player Controller` :type "/Game/Programming/Blueprints/Core/BP_PlayerController Object Reference"))
  (bind _is_paused (`self.Is Paused`))
  (if _is_paused
    (bind _output_get (set `self.Is Paused` (not _is_paused) :!label _label))
    (`AudioComponent.SetPaused` (`self.Audio`) _output_get)
    (else
      (`self.Next Playlist`)
      (if (== (`self.Playlist ID`) 0)
        (goto _label)))))

(event `self.Audio.OnAudioFinished`
  (`self.Next Sound`)
  (`AudioComponent.Play` (`self.Audio`) 0.0))

(fn `Next Playlist`
  (set `self.Playlist ID` (mod (+ (`self.Playlist ID`) 1) (`KismetArrayLibrary.Array_Length` (`/Game/Programming/Blueprints/Data/BP_JukeboxData.Playlists` (`self.Data`)))))
  (set `self.Sound ID` -1)
  (`self.Next Sound`))

(fn `Next Sound`
  (bind _sounds (break `/Game/Programming/Blueprints/Data/S_Playlist` (`|GetArrayItem` (`/Game/Programming/Blueprints/Data/BP_JukeboxData.Playlists` (`self.Data`)) (`self.Playlist ID`))))
  (bind _output_get (set `self.Sound ID` (mod (+ (`self.Sound ID`) 1) (`KismetArrayLibrary.Array_Length` _sounds))))
  (`AudioComponent.SetSound` (`self.Audio`) (`|GetArrayItem` _sounds _output_get)))

(fn `UserConstructionScript`)