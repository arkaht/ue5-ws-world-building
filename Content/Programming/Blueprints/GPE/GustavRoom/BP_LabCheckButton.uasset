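; Interactable check button for a lab puzzle in the Gustav room that validates the objects on a set of BP_LabDropTable actors.
; On interact it counts the tables whose CheckObjectType passes and compares the count to the table total.
; A full match switches to the green light, while a miss shows red for LightDelay before restoring the base light.
; Lights toggle through intensity, using values cached at BeginPlay.
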(event `self.ReceiveBeginPlay`
  (bind _lightcomponent (`Light.LightComponent` (`self.GreenLight`)))
  (bind _lightcomponent_2 (`Light.LightComponent` (`self.RedLight`)))
  (set `self.BL_Intensity` (`LightComponentBase.Intensity` (`Light.LightComponent` (`self.BaseLight`))))
  (set `self.GL_Intensity` (`LightComponentBase.Intensity` _lightcomponent))
  (`LightComponent.SetIntensity` _lightcomponent 0.0)
  (set `self.RL_Intensity` (`LightComponentBase.Intensity` _lightcomponent_2))
  (`LightComponent.SetIntensity` _lightcomponent_2 0.0))

(event `self.InteractionComponent.On Interact`
  (params (`Player Controller` :type "/Game/Programming/Blueprints/Core/BP_PlayerController Object Reference"))
  (set `self.CorrectCounter` 0)
  (set `self.CorrectNumber` (`KismetArrayLibrary.Array_Length` (`self.TableToCheck`)))
  (for _array_element (`self.TableToCheck`)
    (bind _asbp_lab_drop_table (cast `/Game/Programming/Blueprints/GPE/GustavRoom/BP_LabDropTable` _array_element))
    (bind _isobjectmatching_ (`/Game/Programming/Blueprints/GPE/GustavRoom/BP_LabDropTable.CheckObjectType` _asbp_lab_drop_table))
    (if _isobjectmatching_
      (set `self.CorrectCounter` (+ (`self.CorrectCounter`) 1))))
  (if (== (`self.CorrectCounter`) (`self.CorrectNumber`))
    (`LightComponent.SetIntensity` (`Light.LightComponent` (`self.BaseLight`)) 0.0)
    (`LightComponent.SetIntensity` (`Light.LightComponent` (`self.GreenLight`)) (`self.GL_Intensity`))
    (`LightComponent.SetIntensity` (`Light.LightComponent` (`self.RedLight`)) 0.0)
    (else
      (`LightComponent.SetIntensity` (`Light.LightComponent` (`self.BaseLight`)) 0.0)
      (`LightComponent.SetIntensity` (`Light.LightComponent` (`self.GreenLight`)) 0.0)
      (`LightComponent.SetIntensity` (`Light.LightComponent` (`self.RedLight`)) (`self.RL_Intensity`))
      (`KismetSystemLibrary.Delay` (`self.LightDelay`))
      (`LightComponent.SetIntensity` (`Light.LightComponent` (`self.BaseLight`)) (`self.BL_Intensity`))
      (`LightComponent.SetIntensity` (`Light.LightComponent` (`self.GreenLight`)) 0.0)
      (`LightComponent.SetIntensity` (`Light.LightComponent` (`self.RedLight`)) 0.0))))

(fn `UserConstructionScript`)