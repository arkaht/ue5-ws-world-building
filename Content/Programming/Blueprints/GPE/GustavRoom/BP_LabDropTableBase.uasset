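; BP_LabDropTableBase is a lab table where the player can drop a held object.
; On BeginPlay it caches the player, the AreaToDrop location and all actors tagged "Shape".
; Collider overlap lets a grabbing player drop at that location if the table is free.
; When the player leaves, it revokes dropping and flags the table occupied if any shape lies within a small radius of the spot.
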(event `self.ReceiveBeginPlay`
  (set `self.AreaToDropLocation` (`SceneComponent.K2_GetComponentLocation` (`self.AreaToDrop`)))
  (bind _returnvalue (`GameplayStatics.GetActorOfClass` "/Game/Programming/Blueprints/Core/BP_Player.BP_Player_C"))
  (set `self.Player` _returnvalue)
  (bind _outactors (`GameplayStatics.GetAllActorsWithTag` "Shape"))
  (set `self.Shapes` _outactors))

(event `self.Collider.OnComponentBeginOverlap`
  (params (OverlappedComponent :type "PrimitiveComponent Object Reference") (OtherActor :type "Actor Object Reference") (OtherComp :type "PrimitiveComponent Object Reference") (OtherBodyIndex :type Integer) (bFromSweep :type Boolean) (SweepResult :type "HitResult Structure (by ref)"))
  (if (`/Game/Programming/Blueprints/Core/BP_Player.IsGrabbingObject?` (`self.Player`))
    (if (not (`self.HasObjectPlacedOnSelf?`))
      (set `/Game/Programming/Blueprints/Core/BP_Player.CanDropHoldingObject?` true (`self.Player`))
      (set `/Game/Programming/Blueprints/Core/BP_Player.AreaToDropObject` (`self.AreaToDropLocation`) (`self.Player`)))))

(event `self.Collider.OnComponentEndOverlap`
  (params (OverlappedComponent :type "PrimitiveComponent Object Reference") (OtherActor :type "Actor Object Reference") (OtherComp :type "PrimitiveComponent Object Reference") (OtherBodyIndex :type Integer))
  (if (== OtherActor (`self.Player`))
    (set `/Game/Programming/Blueprints/Core/BP_Player.CanDropHoldingObject?` false (`self.Player`))
    (for _array_element (`self.Shapes`)
      (if (< (`KismetMathLibrary.Vector_Distance` (`self.K2_GetActorLocation` _array_element) (`self.AreaToDropLocation`)) 30.0)
        (set `self.HasObjectPlacedOnSelf?` true)
        (break)
        (else
          (set `self.HasObjectPlacedOnSelf?` false))))))

(fn `UserConstructionScript`)