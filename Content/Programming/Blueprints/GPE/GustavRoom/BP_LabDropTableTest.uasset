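; Test lab drop table that lets the player place a held object and judges whether the shape on it is the correct type.
; Overlapping the collider while the player holds something enables dropping at AreaToDrop's location.
; Any end overlap rescans "Shape"-tagged actors cached at BeginPlay by distance to that spot, storing the CorrectType match for CheckObjectType.
; CheckPlayerHasShape reports a held shape; the delamerde graphs and older checks are dead code.
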(event `self.ReceiveTick`
  (params (DeltaSeconds :type "Float (single-precision)")))

(event `self.ReceiveBeginPlay`
  (set `self.AreaToDropLocation` (`SceneComponent.K2_GetComponentLocation` (`self.AreaToDrop`)))
  (bind _asbp_player (cast `/Game/Programming/Blueprints/Core/BP_Player` (`GameplayStatics.GetPlayerPawn` 0)))
  (set `self.Player` _asbp_player)
  (bind _outactors (`GameplayStatics.GetAllActorsWithTag` "Shape"))
  (set `self.Shapes` _outactors))

(event `self.Collider.OnComponentBeginOverlap`
  (params (OverlappedComponent :type "PrimitiveComponent Object Reference") (OtherActor :type "Actor Object Reference") (OtherComp :type "PrimitiveComponent Object Reference") (OtherBodyIndex :type Integer) (bFromSweep :type Boolean) (SweepResult :type "HitResult Structure (by ref)"))
  (bind _player (`self.Player`))
  (if (`/Game/Programming/Blueprints/Core/BP_Player.IsGrabbingObject?` (`self.Player`))
    (set `/Game/Programming/Blueprints/Core/BP_Player.CanDropHoldingObject?` true _player)
    (set `/Game/Programming/Blueprints/Core/BP_Player.AreaToDropObject` (`self.AreaToDropLocation`) _player)))

(event `self.Collider.OnComponentEndOverlap`
  (params (OverlappedComponent :type "PrimitiveComponent Object Reference") (OtherActor :type "Actor Object Reference") (OtherComp :type "PrimitiveComponent Object Reference") (OtherBodyIndex :type Integer))
  (bind _player (`self.Player`))
  (`|ExecutionSequence`
    (:`then_0`
      (for _array_element (`self.Shapes`)
        (if (< (`KismetMathLibrary.Vector_Distance` (`self.K2_GetActorLocation` _array_element) (`self.AreaToDropLocation`)) 30.0)
          (bind _asbp_lab_shapes (cast `/Game/Programming/Blueprints/GPE/GustavRoom/BP_LabShapes` _array_element))
          (set `self.IsObjectRight?` (`|EnumEquality` (`/Game/Programming/Blueprints/GPE/GustavRoom/BP_LabShapes.Shape` _asbp_lab_shapes) (`self.CorrectType`)))
          (break)
          (else
            (set `self.IsObjectRight?` false)))))
    (:`then_1`
      (if (== OtherActor _player)
        (set `/Game/Programming/Blueprints/Core/BP_Player.CanDropHoldingObject?` false _player)))))

(fn `CheckObjectType`
  (returns (`IsObjectMatching?` :type Boolean))
  (return (`self.IsObjectRight?`)))

(fn `CheckPlayerHasShape`
  (returns (IsValid :type Boolean))
  (bind _grabbedactor (`/Game/Programming/Blueprints/Core/BP_Player.GrabbedActor` (`self.Player`)))
  (`/Engine/EditorBlueprintResources/StandardMacros.IsValid` _grabbedactor
    (:`Is Valid`
      (return (and (`/Game/Programming/Blueprints/Core/BP_Player.IsGrabbingObject?` (`self.Player`)) (`self.ActorHasTag` _grabbedactor "Shape"))))))

(fn `UserConstructionScript`)