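; BP_LabShapesFucked is a lab shape the player can pick up and drop, with mesh and material applied on BeginPlay.
; Interaction toggles between pickup and drop by setting grab state on BP_Player; dropping also calls OnTrophyInteraction and moves the shape to the player's location.
; Collider overlaps and pickup/drop changes are reported to the BP_LabCarryManager found in the level.
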(event `self.ReceiveBeginPlay`
  (bind _body (`self.Body`))
  (`|ExecutionSequence`
    (:`then_0`
      (`StaticMeshComponent.SetStaticMesh` _body (`self.Mesh`))
      (`PrimitiveComponent.SetMaterial` _body 0 (`self.MeshColor`))
      (bind _asbp_player (cast `/Game/Programming/Blueprints/Core/BP_Player` (`Controller.K2_GetPawn` (`GameplayStatics.GetPlayerController` 0))))
      (set `self.PlayerRef` _asbp_player)
      (bind _returnvalue (`GameplayStatics.GetActorOfClass` "/Game/Programming/Blueprints/GPE/GustavRoom/BP_LabCarryManager.BP_LabCarryManager_C"))
      (set `self.ShapeManager` _returnvalue))))

(event `self.BP_InteractionComponent.On Interact`
  (params (`Player Controller` :type "/Game/Programming/Blueprints/Core/BP_PlayerController Object Reference"))
  (bind _asbp_player (cast `/Game/Programming/Blueprints/Core/BP_Player` (`Controller.K2_GetPawn` `Player Controller`)))
  (set `self.PlayerRef` _asbp_player)
  (if (`self.IsPickedUp?`)
    (`self.DropMe`)
    (set `self.IsPickedUp?` false)
    (`/Game/Programming/Blueprints/GPE/GustavRoom/BP_LabCarryManager.PlayerDropShape` (`self.ShapeManager`))
    (else
      (`self.PlayerPickUpSelf`)
      (set `self.IsPickedUp?` true)
      (`/Game/Programming/Blueprints/GPE/GustavRoom/BP_LabCarryManager.PlayerPickUpShape` (`self.ShapeManager`) null))))

(event `self.Collider.OnComponentBeginOverlap`
  (params (OverlappedComponent :type "PrimitiveComponent Object Reference") (OtherActor :type "Actor Object Reference") (OtherComp :type "PrimitiveComponent Object Reference") (OtherBodyIndex :type Integer) (bFromSweep :type Boolean) (SweepResult :type "HitResult Structure (by ref)"))
  (if (== OtherActor (`self.PlayerRef`))
    (`/Game/Programming/Blueprints/GPE/GustavRoom/BP_LabCarryManager.PlayerOnShape` (`self.ShapeManager`) self)))

(event `self.Collider.OnComponentEndOverlap`
  (params (OverlappedComponent :type "PrimitiveComponent Object Reference") (OtherActor :type "Actor Object Reference") (OtherComp :type "PrimitiveComponent Object Reference") (OtherBodyIndex :type Integer))
  (if (== OtherActor (`self.PlayerRef`))
    (`/Game/Programming/Blueprints/GPE/GustavRoom/BP_LabCarryManager.PlayerLeaveShape` (`self.ShapeManager`))))

(fn `DropMe`
  (bind _playerref (`self.PlayerRef`))
  (set `/Game/Programming/Blueprints/Core/BP_Player.IsGrabbingObject?` true _playerref)
  (set `/Game/Programming/Blueprints/Core/BP_Player.CanDropHoldingObject?` true _playerref)
  (`/Game/Programming/Blueprints/Core/BP_Player.OnTrophyInteraction` (`self.PlayerRef`) self)
  (`self.K2_SetActorLocation` (`self.K2_GetActorLocation` (`self.PlayerRef`))))

(fn `PlayerPickUpSelf`
  (bind _playerref (`self.PlayerRef`))
  (set `/Game/Programming/Blueprints/Core/BP_Player.IsGrabbingObject?` true _playerref)
  (set `/Game/Programming/Blueprints/Core/BP_Player.ActorToPick` self _playerref)
  (set `/Game/Programming/Blueprints/Core/BP_Player.GrabbedActor` self _playerref))

(fn `UserConstructionScript`)