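; Drop table in Gustav's lab room that lets the player set down a carried shape at a fixed spot cached on BeginPlay.
; When a held Shape-tagged actor enters the collider and no object occupies it, the table records it and passes the player drop permission and location.
; Any end overlap clears the incoming object and revokes permission.
; Helper functions check the shape against CorrectType and whether the player holds a shape.
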(event `self.ReceiveBeginPlay`
  (set `self.AreaToDropLocation` (`SceneComponent.K2_GetComponentLocation` (`self.AreaToDrop`)))
  (bind _asbp_player (cast `/Game/Programming/Blueprints/Core/BP_Player` (`GameplayStatics.GetPlayerPawn` 0)))
  (set `self.Player` _asbp_player))

(event `self.Collider.OnComponentBeginOverlap`
  (params (OverlappedComponent :type "PrimitiveComponent Object Reference") (OtherActor :type "Actor Object Reference") (OtherComp :type "PrimitiveComponent Object Reference") (OtherBodyIndex :type Integer) (bFromSweep :type Boolean) (SweepResult :type "HitResult Structure (by ref)"))
  (bind _player (`self.Player`))
  (if (`/Game/Programming/Blueprints/Core/BP_Player.IsGrabbingObject?` (`self.Player`))
    (if (`self.ActorHasTag` OtherActor "Shape")
      (bind _output_get (set `self.ObjectComing` OtherActor))
      (`/Engine/EditorBlueprintResources/StandardMacros.IsValid` (`self.ObjectStaying`)
        (:`Is Not Valid`
          (set `self.ObjectStaying` _output_get)
          (set `/Game/Programming/Blueprints/Core/BP_Player.CanDropHoldingObject?` true _player)
          (set `/Game/Programming/Blueprints/Core/BP_Player.AreaToDropObject` (`self.AreaToDropLocation`) _player))))))

(event `self.Collider.OnComponentEndOverlap`
  (params (OverlappedComponent :type "PrimitiveComponent Object Reference") (OtherActor :type "Actor Object Reference") (OtherComp :type "PrimitiveComponent Object Reference") (OtherBodyIndex :type Integer))
  (bind _objectcoming (`self.ObjectComing`))
  (`|ExecutionSequence`
    (:`then_0`
      (if (`self.ActorHasTag` OtherActor "Shape")
        (`|ExecutionSequence`
          (:`then_0`
            (if (== (`self.ObjectStaying`) OtherActor)
              (`/Engine/EditorBlueprintResources/StandardMacros.IsValid` _objectcoming
                (:`Is Valid`
                  (set `self.ObjectStaying` _objectcoming))
                (:`Is Not Valid`
                  (set `self.ObjectStaying` null)))))
          (:`then_1`
            (set `self.ObjectComing` null :!label _label)
            (set `/Game/Programming/Blueprints/Core/BP_Player.CanDropHoldingObject?` false (`self.Player`))))))
    (:`then_1`
      (goto _label))))

(fn `CheckObjectType`
  (returns (`IsObjectMatching?` :type Boolean))
  (bind _asbp_lab_shapes (cast `/Game/Programming/Blueprints/GPE/GustavRoom/BP_LabShapes` (`self.ObjectStaying`)))
  (return (`|EnumEquality` (`/Game/Programming/Blueprints/GPE/GustavRoom/BP_LabShapes.Shape` _asbp_lab_shapes) (`self.CorrectType`))))

(fn `CheckPlayerHasShape`
  (returns (IsValid :type Boolean))
  (bind _grabbedactor (`/Game/Programming/Blueprints/Core/BP_Player.GrabbedActor` (`self.Player`)))
  (`/Engine/EditorBlueprintResources/StandardMacros.IsValid` _grabbedactor
    (:`Is Valid`
      (return (and (`/Game/Programming/Blueprints/Core/BP_Player.IsGrabbingObject?` (`self.Player`)) (`self.ActorHasTag` _grabbedactor "Shape"))))))

(fn `UserConstructionScript`)