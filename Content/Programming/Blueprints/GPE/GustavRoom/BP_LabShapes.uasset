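; Pickable lab shape for the Gustav room, with a configurable mesh and color material applied on BeginPlay.
; On interact, it passes itself to BP_Player's trophy interaction, then notifies every BP_LabDropTable and the BP_LabCheckButton of a shape drop.
; An older pickup/drop toggle using DropMe and PlayerPickUpSelf remains in the graph but is disconnected and never runs.
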(event `self.ReceiveBeginPlay`
  (bind _body (`self.Body`))
  (`|ExecutionSequence`
    (:`then_0`
      (`StaticMeshComponent.SetStaticMesh` _body (`self.Mesh`))
      (`PrimitiveComponent.SetMaterial` _body 0 (`self.MeshColor`))
      (bind _asbp_player (cast `/Game/Programming/Blueprints/Core/BP_Player` (`Controller.K2_GetPawn` (`GameplayStatics.GetPlayerController` 0))))
      (set `self.PlayerRef` _asbp_player)
      (`GameplayStatics.GetActorOfClass` "/Game/Programming/Blueprints/GPE/GustavRoom/BP_LabCarryManager.BP_LabCarryManager_C"))))

(event `self.BP_InteractionComponent.On Interact`
  (params (`Player Controller` :type "/Game/Programming/Blueprints/Core/BP_PlayerController Object Reference"))
  (bind _asbp_player (cast `/Game/Programming/Blueprints/Core/BP_Player` (`Controller.K2_GetPawn` `Player Controller`)))
  (bind _output_get (set `self.PlayerRef` _asbp_player))
  (`/Game/Programming/Blueprints/Core/BP_Player.OnTrophyInteraction` _output_get self)
  (bind _outactors (`GameplayStatics.GetAllActorsOfClass` "/Game/Programming/Blueprints/GPE/GustavRoom/BP_LabDropTable.BP_LabDropTable_C"))
  (for _array_element _outactors
    (`/Game/Programming/Blueprints/GPE/GustavRoom/BP_LabDropTable.OnShapeDrop` _array_element))
  (bind _returnvalue (`GameplayStatics.GetActorOfClass` "/Game/Programming/Blueprints/GPE/GustavRoom/BP_LabCheckButton.BP_LabCheckButton_C"))
  (`/Game/Programming/Blueprints/GPE/GustavRoom/BP_LabCheckButton.OnShapeDropPanel` _returnvalue))

(fn `DropMe`
  (bind _playerref (`self.PlayerRef`))
  (set `/Game/Programming/Blueprints/Core/BP_Player.IsGrabbingObject?` true _playerref)
  (set `/Game/Programming/Blueprints/Core/BP_Player.CanDropHoldingObject?` true _playerref)
  (`/Game/Programming/Blueprints/Core/BP_Player.OnTrophyInteraction` (`self.PlayerRef`) self)
  (`self.K2_SetActorLocation` (`self.K2_GetActorLocation` (`self.PlayerRef`))))

(fn `PlayerPickUpSelf`
  (bind _playerref (`self.PlayerRef`))
  (set `/Game/Programming/Blueprints/Core/BP_Player.IsGrabbingObject?` true _playerref)
  (set `/Game/Programming/Blueprints/Core/BP_Player.ActorToPick` self _playerref)
  (set `/Game/Programming/Blueprints/Core/BP_Player.GrabbedActor` self _playerref))

(fn `UserConstructionScript`)