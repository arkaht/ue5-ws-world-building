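; BP_LabCarryManager tracks which shape the player carries and which shape they stand on in the lab room.
; Pick-up stores the held shape, while the on-shape and leave-shape functions record or clear the floor shape and print debug messages.
; Dropping clears the holding flag, then immediately picks up the floor shape if it is valid and differs from the one just held, allowing a swap.
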(fn `PlayerDropShape`
  (bind _shapeonfloor (`self.ShapeOnFloor`))
  (set `self.IsHoldingACube?` false)
  (if (`self.IsShapeOnFloor?`)
    (if (not (== (`self.ShapeOnFloor`) (`self.ShapeInHands`)))
      (`/Engine/EditorBlueprintResources/StandardMacros.IsValid` _shapeonfloor
        (:`Is Valid`
          (`/Game/Programming/Blueprints/GPE/GustavRoom/BP_LabShapes.PlayerPickUpSelf` _shapeonfloor)
          (set `/Game/Programming/Blueprints/GPE/GustavRoom/BP_LabShapes.IsPickedUp?` true _shapeonfloor)
          (`self.PlayerPickUpShape` _shapeonfloor))))))

(fn `PlayerLeaveShape`
  (set `self.ShapeOnFloor` null)
  (set `self.IsShapeOnFloor?` false)
  (`KismetSystemLibrary.PrintString` "player leave shape"))

(fn `PlayerOnShape`
  (params (Shape :type "/Game/Programming/Blueprints/GPE/GustavRoom/BP_LabShapes Object Reference"))
  (set `self.ShapeOnFloor` Shape)
  (set `self.IsShapeOnFloor?` true)
  (`KismetSystemLibrary.PrintString` "player on shape"))

(fn `PlayerPickUpShape`
  (params (ShapePicked :type "/Game/Programming/Blueprints/GPE/GustavRoom/BP_LabShapes Object Reference"))
  (set `self.IsHoldingACube?` true)
  (set `self.ShapeInHands` ShapePicked))

(fn `UserConstructionScript`)