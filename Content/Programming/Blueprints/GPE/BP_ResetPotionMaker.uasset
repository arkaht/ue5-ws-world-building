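; BP_ResetPotionMaker is an interactable that broadcasts OnReset, presumably to reset the potion maker, using an animated cube.
; On interact it ignores the player's move input, with no re-enable in this graph, and slides the cube along world X by DistanceLerp.
; When that timeline finishes it calls OnReset, and a second timeline slides the cube back.
; CanInteract requires a valid player with no grabbed actor.
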(event `self.BP_InteractionComponent.On Interact`
  (params (`Player Controller` :type "/Game/Programming/Blueprints/Core/BP_PlayerController Object Reference"))
  (`Controller.SetIgnoreMoveInput` `Player Controller` true)
  (set `self.SaveLocation` (`SceneComponent.GetSocketLocation` (`self.Cube`) "None"))
  (bind (_direction _newtrack_0) (`Timeline|Timeline_0` :!via `PlayFromStart`)
    (:`Update`
      (`SceneComponent.K2_SetWorldLocation` (`self.Cube`) (+ (`self.SaveLocation`) (`KismetMathLibrary.MakeVector` (`KismetMathLibrary.Lerp` 0.0 (`self.DistanceLerp`) _newtrack_0))) false false))
    (:`Finished`
      (`self.On Reset`)
      (bind (_direction_2 _newtrack_0_2) (`Timeline|Timeline_1` :!via `PlayFromStart`)
        (:`Update`
          (`SceneComponent.K2_SetWorldLocation` (`self.Cube`) (+ (`self.SaveLocation`) (`KismetMathLibrary.MakeVector` (`KismetMathLibrary.Lerp` (`self.DistanceLerp`) 0.0 _newtrack_0_2))) false false))))))

(fn `Can Interact`
  (params (`Player Controller` :type "/Game/Programming/Blueprints/Core/BP_PlayerController Object Reference"))
  (returns (`Can Interact` :type Boolean))
  (bind _bp_player (`/Game/Programming/Blueprints/Core/BP_PlayerController.BP Player` `Player Controller`))
  (`/Engine/EditorBlueprintResources/StandardMacros.IsValid` _bp_player
    (:`Is Valid`
      (return (not (`KismetSystemLibrary.IsValid` (`/Game/Programming/Blueprints/Core/BP_Player.GrabbedActor` _bp_player)))))))

(fn `UserConstructionScript`)