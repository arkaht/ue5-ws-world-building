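; Interactable that starts and runs a "red light, green light" dance-floor minigame.
; Tick uses DoOnce and Delay loops to alternate music-on movement and paused freeze phases, syncing traffic-light spheres, spotlights and randomized floor tiles.
; After a reaction delay, player velocity is checked and movement means losing.
; NextStep advances step lights up to the win, where Stop resets the set and has BP_RandomOjectSpawner spawn a trophy.
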(event `self.ReceiveTick`
  (params (DeltaSeconds :type "Float (single-precision)"))
  (if (`self.isGameWin`)
    ;[1 0 0.5314] Debugging
    (`/Engine/EditorBlueprintResources/StandardMacros.DoOnce` false
      (:`Completed`
        (`KismetSystemLibrary.Delay` 1.0)
        (for _array_element (`self.DanceFloor`)
          (bind _asstatic_mesh_actor (cast `StaticMeshActor` _array_element))
          (`MeshComponent.SetVectorParameterValueOnMaterials` (`StaticMeshActor.StaticMeshComponent` _asstatic_mesh_actor) "Param" (0.1 0.1 0.1)))))
    (else
      (`|ExecutionSequence`
        (:`then_0`
          (if (`self.isGameStarted`)
            (`|ExecutionSequence`
              (:`then_0`
                ;[0 0.586 1] Delay while the player can move, and can't move. The game stop if the player move when he can't
                (`/Engine/EditorBlueprintResources/StandardMacros.DoOnce` false :!label _label
                  (:`Completed`
                    (set `self.isLooping` true)
                    (set `self.CanMoveTimer` 4.0)
                    (set `self.canMove?` true)
                    (`AudioComponent.SetPaused` (`self.Music_OneTwoThree`) false)
                    (`KismetSystemLibrary.Delay` (`self.CanMoveTimer`))
                    (set `self.canMove?` false)
                    (`AudioComponent.SetPaused` (`self.Music_OneTwoThree`) true)
                    (`KismetSystemLibrary.Delay` (`self.ReactionTime`))
                    (set `self.checkPlayer` true)
                    (bind _output_get (set `self.CanMoveTimer` 1.0))
                    (`KismetSystemLibrary.Delay` _output_get)
                    (set `self.checkPlayer` false)
                    (goto _label :!via `Reset`))))
              (:`then_1`
                ;[0 0.586 1] Change SphereColor
                (if (`self.canMove?`)
                  (`/Engine/EditorBlueprintResources/StandardMacros.DoOnce` false :!label _label_2
                    (:`Completed`
                      (for _array_element_2 (`self.Actors Light Array`)
                        (`MeshComponent.SetVectorParameterValueOnMaterials` (`/Game/Programming/Blueprints/GPE/BP_123_Sun_Game.Green_Sphere` _array_element_2) "Emissive Color" (0.0 100.0 0.0))
                        (`MeshComponent.SetVectorParameterValueOnMaterials` (`/Game/Programming/Blueprints/GPE/BP_123_Sun_Game.Red_Sphere` _array_element_2) "Emissive Color" (0.0 0.0 0.0)))
                      (`self.BlueTile`)
                      (`KismetSystemLibrary.Delay` (/ (`self.CanMoveTimer`) 4.0))
                      (`self.BlueTile`)
                      (`KismetSystemLibrary.Delay` (/ (`self.CanMoveTimer`) 4.0))
                      (for _array_element_3 (`self.Actors Light Array`)
                        (`MeshComponent.SetVectorParameterValueOnMaterials` (`/Game/Programming/Blueprints/GPE/BP_123_Sun_Game.Yellow_Sphere` _array_element_3) "Emissive Color" (100.0 100.0 0.0))
                        (`MeshComponent.SetVectorParameterValueOnMaterials` (`/Game/Programming/Blueprints/GPE/BP_123_Sun_Game.Green_Sphere` _array_element_3) "Emissive Color" (0.0 0.0 0.0)))
                      (`self.PinkTile`)
                      (`KismetSystemLibrary.Delay` (/ (`self.CanMoveTimer`) 4.0))
                      (`self.PinkTile`)
                      (goto _label_3 :!via `Reset`)))
                  (else
                    (`/Engine/EditorBlueprintResources/StandardMacros.DoOnce` false :!label _label_3
                      (:`Completed`
                        (for _array_element_4 (`self.Actors Light Array`)
                          (`MeshComponent.SetVectorParameterValueOnMaterials` (`/Game/Programming/Blueprints/GPE/BP_123_Sun_Game.Red_Sphere` _array_element_4) "Emissive Color" (100.0 0.0 0.0))
                          (`MeshComponent.SetVectorParameterValueOnMaterials` (`/Game/Programming/Blueprints/GPE/BP_123_Sun_Game.Yellow_Sphere` _array_element_4) "Emissive Color" (0.0 0.0 0.0))
                          (`MeshComponent.SetVectorParameterValueOnMaterials` (`/Game/Programming/Blueprints/GPE/BP_123_Sun_Game.Green_Sphere` _array_element_4) "Emissive Color" (0.0 0.0 0.0)))
                        (`self.RedTile`)
                        (goto _label_2 :!via `Reset`))))))
              (:`then_2`
                ;[0 0.586 1] Check the player is moving
                (if (`self.checkPlayer`)
                  (`self.CheckPlayerVelocity`)))
              (:`then_3`
                ;[0 0.586 1] Change Lights Color
                (if (`self.canMove?`)
                  (`/Engine/EditorBlueprintResources/StandardMacros.DoOnce` false :!label _label_4
                    (:`Completed`
                      (`GameplayStatics.PlaySound2D` "/Game/Design/Sounds/Bips/BipBoupA.BipBoupA" 1.0 1.0 0.0 null null false)
                      (for _array_element_5 (`self.SpotLights`)
                        (`LightComponent.SetLightColor` (`SpotLight.SpotLightComponent` _array_element_5) (struct :`G` 1.0 :`A` 1.0) true))
                      (`KismetSystemLibrary.Delay` (/ (`self.CanMoveTimer`) 2.0))
                      (`GameplayStatics.PlaySound2D` "/Game/Design/Sounds/Bips/BipBoupA.BipBoupA" 1.0 1.0 0.0 null null false)
                      (for _array_element_6 (`self.SpotLights`)
                        (`LightComponent.SetLightColor` (`SpotLight.SpotLightComponent` _array_element_6) (struct :`R` 1.0 :`G` 1.0 :`A` 1.0) true))
                      (goto _label_5 :!via `Reset`)))
                  (else
                    (`/Engine/EditorBlueprintResources/StandardMacros.DoOnce` false :!label _label_5
                      (:`Completed`
                        (`GameplayStatics.PlaySound2D` "/Game/Design/Sounds/Bips/BipBoupC.BipBoupC" 1.0 1.0 0.0 null null false)
                        (for _array_element_7 (`self.SpotLights`)
                          (`LightComponent.SetLightColor` (`SpotLight.SpotLightComponent` _array_element_7) (struct :`R` 1.0 :`A` 1.0) true))
                        (goto _label_4 :!via `Reset`)))))))))
        (:`then_1`
          (if (< (`self.StepCount`) 3)
            (`/Engine/EditorBlueprintResources/StandardMacros.DoOnce` false :!label _label_6
              (:`Completed`
                (bind (_direction _light_intensity) (`Timeline|Timeline_0` :!via `PlayFromStart`)
                  (:`Update`
                    (`LightComponent.SetIntensity` (`Light.LightComponent` (`|GetArrayItem` (`self.StepsLight`) (`self.StepCount`))) (* _light_intensity 160.0)))
                  (:`Finished`
                    (goto _label_6 :!via `Reset`)))))))))))

(event `self.BP_InteractionComponent.On Interact`
  (params (`Player Controller` :type "/Game/Programming/Blueprints/Core/BP_PlayerController Object Reference"))
  ;[0 0.586 1] Start the Game
  (if (`self.isGameWin`)
    _
    (elif (not (`self.isGameStarted`))
      (set `self.Player` (`/Game/Programming/Blueprints/Core/BP_PlayerController.BP Player` `Player Controller`))
      (set `self.isGameStarted` true)
      (`AudioComponent.Play` (`self.Music_OneTwoThree`) 0.0)
      (`self.NextStep`))))

(event `self.ReceiveBeginPlay`
  ;[0 0.586 1] Event Begin
  (`AudioComponent.Stop` (`self.Music_OneTwoThree`))
  (set `self.isGameWin` false))

(fn `BlueTile`
  (for _array_element (`self.DanceFloor`)
    (if (> (`KismetMathLibrary.RandomInteger` 3) 0)
      (bind _asstatic_mesh_actor (cast `StaticMeshActor` _array_element))
      (`MeshComponent.SetVectorParameterValueOnMaterials` (`StaticMeshActor.StaticMeshComponent` _asstatic_mesh_actor) "Param" (0.0 5.0 0.0))
      (else
        (bind _asstatic_mesh_actor_2 (cast `StaticMeshActor` _array_element))
        (`MeshComponent.SetVectorParameterValueOnMaterials` (`StaticMeshActor.StaticMeshComponent` _asstatic_mesh_actor_2) "Param" (0.01 0.01 0.01))))))

(fn `CheckPlayerVelocity`
  (bind (_returnvalue_x _returnvalue_y) (`KismetMathLibrary.BreakVector` (`self.GetVelocity` (`self.Player`))))
  (if (not (and (< (`KismetMathLibrary.Abs` _returnvalue_x) 0.25) (< (`KismetMathLibrary.Abs` _returnvalue_y) 0.25)))
    (`KismetSystemLibrary.PrintString` "DIE" true true (struct :`R` 1.0 :`B` 0.084265 :`A` 1.0) 0.5 "1")
    (`self.Stop`)
    (set `self.isGameStarted` false)))

(fn `NextStep`
  (`LightComponent.SetIntensity` (`Light.LightComponent` (`|GetArrayItem` (`self.StepsLight`) (`self.StepCount`))) 0.0)
  (set `self.StepCount` (+ (`self.StepCount`) 1))
  (if (< (`self.StepCount`) 4)
    (`LightComponent.SetIntensity` (`Light.LightComponent` (`|GetArrayItem` (`self.StepsLight`) (`self.StepCount`))) 160.0))
  (if (>= (`self.StepCount`) 4)
    (set `self.isGameWin` true)
    (`self.Stop`)
    (set `self.isGameStarted` false)))

(fn `PinkTile`
  (for _array_element (`self.DanceFloor`)
    (if (> (`KismetMathLibrary.RandomInteger` 3) 0)
      (bind _asstatic_mesh_actor (cast `StaticMeshActor` _array_element))
      (`MeshComponent.SetVectorParameterValueOnMaterials` (`StaticMeshActor.StaticMeshComponent` _asstatic_mesh_actor) "Param" (4.0 4.0 0.0))
      (else
        (bind _asstatic_mesh_actor_2 (cast `StaticMeshActor` _array_element))
        (`MeshComponent.SetVectorParameterValueOnMaterials` (`StaticMeshActor.StaticMeshComponent` _asstatic_mesh_actor_2) "Param" (0.01 0.01 0.01))))))

(fn `RedTile`
  (for _array_element (`self.DanceFloor`)
    (if (> (`KismetMathLibrary.RandomInteger` 3) 0)
      (bind _asstatic_mesh_actor (cast `StaticMeshActor` _array_element))
      (`MeshComponent.SetVectorParameterValueOnMaterials` (`StaticMeshActor.StaticMeshComponent` _asstatic_mesh_actor) "Param" (8.0 0.0 0.0))
      (else
        (bind _asstatic_mesh_actor_2 (cast `StaticMeshActor` _array_element))
        (`MeshComponent.SetVectorParameterValueOnMaterials` (`StaticMeshActor.StaticMeshComponent` _asstatic_mesh_actor_2) "Param" (0.01 0.01 0.01))))))

(fn `Stop`
  (if (`self.isGameStarted`)
    (if (`self.isGameWin`)
      (`AudioComponent.SetPaused` (`self.Music_OneTwoThree`) true)
      (`GameplayStatics.PlaySound2D` "/Game/Design/Sounds/Others/YouWin.YouWin" 1.0 1.0 0.0 null null)
      (bind _returnvalue (`GameplayStatics.GetActorOfClass` "/Game/Programming/Blueprints/Objects/BP_RandomOjectSpawner.BP_RandomOjectSpawner_C"))
      (`/Game/Programming/Blueprints/Objects/BP_RandomOjectSpawner.Spawn Trophy` _returnvalue 5)
      (else
        (`AudioComponent.SetPaused` (`self.Music_OneTwoThree`) true)
        (`GameplayStatics.PlaySound2D` "/Game/Design/Sounds/Others/LooseSFX.LooseSFX" 1.0 1.0 0.0 null null false)))
    (for _array_element (`self.DanceFloor`)
      (bind _asstatic_mesh_actor (cast `StaticMeshActor` _array_element))
      (`MeshComponent.SetVectorParameterValueOnMaterials` (`StaticMeshActor.StaticMeshComponent` _asstatic_mesh_actor) "Param" (0.1 0.1 0.1)))
    (for _array_element_2 (`self.Actors Light Array`)
      (`MeshComponent.SetVectorParameterValueOnMaterials` (`/Game/Programming/Blueprints/GPE/BP_123_Sun_Game.Red_Sphere` _array_element_2) "Emissive Color" (0.0 0.0 0.0))
      (`MeshComponent.SetVectorParameterValueOnMaterials` (`/Game/Programming/Blueprints/GPE/BP_123_Sun_Game.Yellow_Sphere` _array_element_2) "Emissive Color" (0.0 0.0 0.0))
      (`MeshComponent.SetVectorParameterValueOnMaterials` (`/Game/Programming/Blueprints/GPE/BP_123_Sun_Game.Green_Sphere` _array_element_2) "Emissive Color" (0.0 0.0 0.0)))
    (for _array_element_3 (`self.SpotLights`)
      (`LightComponent.SetLightColor` (`SpotLight.SpotLightComponent` _array_element_3) (struct :`R` 0.043137 :`G` 0.615686 :`B` 1.0 :`A` 1.0) true))
    (for _array_element_4 (`self.StepsLight`)
      (`LightComponent.SetIntensity` (`SpotLight.SpotLightComponent` _array_element_4) 0.0))
    (`LightComponent.SetIntensity` (`Light.LightComponent` (`|GetArrayItem` (`self.StepsLight`))) 160.0)
    (set `self.StepCount` 0)))

(fn `UserConstructionScript`)