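; BP_WTP_Manager is the manager for a bottle puzzle, linking the bottles to a trophy reward.
; On BeginPlay it finds the BP_WTP_Bottles and BP_RandomOjectSpawner actors by class, then passes its three max height values to the bottles as starting heights.
; Its PuzzleFinished function tells the spawner to spawn a trophy; nothing in this Blueprint calls it.
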(event `self.ReceiveBeginPlay`
  (`self.GetReferences`))

(fn `GetReferences`
  (bind _returnvalue (`GameplayStatics.GetActorOfClass` "/Game/Programming/Blueprints/GPE/NewBottlepuzzle/BP_WTP_Bottles.BP_WTP_Bottles_C"))
  (set `self.BottlesReferences` _returnvalue)
  (bind _returnvalue_2 (`GameplayStatics.GetActorOfClass` "/Game/Programming/Blueprints/Objects/BP_RandomOjectSpawner.BP_RandomOjectSpawner_C"))
  (set `self.TrophySpawnerReference` _returnvalue_2)
  (`/Game/Programming/Blueprints/GPE/NewBottlepuzzle/BP_WTP_Bottles.SetStartingBottleHeight` (`self.BottlesReferences`) (`self.MaxAHeight`) (`self.MaxBHeight`) (`self.MaxCHeight`)))

(fn `Puzzle Finished`
  (`/Game/Programming/Blueprints/Objects/BP_RandomOjectSpawner.Spawn Trophy` (`self.TrophySpawnerReference`) 3))

(fn `UserConstructionScript`)