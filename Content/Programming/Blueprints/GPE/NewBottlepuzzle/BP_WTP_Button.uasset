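; BP_WTP_Button is an interactable button in the water bottle puzzle that pours water between two bottles.
; On BeginPlay it finds the BP_WTP_Manager in the level and caches it.
; When its interaction component fires, it asks the manager to transfer water from its FromBottle to its ToBottle, unless the puzzle is already finished.
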(event `self.ReceiveBeginPlay`
  (`self.GetReferences`))

(event `self.BP_InteractionComponent.On Interact`
  (params (`Player Controller` :type "/Game/Programming/Blueprints/Core/BP_PlayerController Object Reference"))
  (if (not (`/Game/Programming/Blueprints/GPE/NewBottlepuzzle/BP_WTP_Manager.isPuzzleFinished` (`self.Water Puzzle Manager`)))
    (`/Game/Programming/Blueprints/GPE/NewBottlepuzzle/BP_WTP_Manager.Transfer Water` (`self.Water Puzzle Manager`) (`self.FromBottle`) (`self.ToBottle`))))

(fn `GetReferences`
  (bind _returnvalue (`GameplayStatics.GetActorOfClass` "/Game/Programming/Blueprints/GPE/NewBottlepuzzle/BP_WTP_Manager.BP_WTP_Manager_C"))
  (set `self.Water Puzzle Manager` _returnvalue))

(fn `UserConstructionScript`)