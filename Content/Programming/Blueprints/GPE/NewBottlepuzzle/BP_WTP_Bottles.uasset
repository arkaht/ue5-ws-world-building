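; Visual actor for the three-bottle liquid puzzle, animating transfers between bottles A, B and C.
; StartTransferVisually stores start and target heights, then Tick lerps each liquid mesh's Z scale over VersingDuration and snaps to the targets.
; A separate function sets bottle heights through Z scale.
; The win check runs as a transfer starts, calling PuzzleFinished on BP_WTP_Manager when B's target is 0.4 and A's nearly matches.
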(event `self.ReceiveBeginPlay`
  (bind _returnvalue (`GameplayStatics.GetActorOfClass` "/Game/Programming/Blueprints/GPE/NewBottlepuzzle/BP_WTP_Manager.BP_WTP_Manager_C"))
  (set `self.Manager ref` _returnvalue))

(event `self.ReceiveTick`
  (params (DeltaSeconds :type "Float (single-precision)"))
  (if (`self.CurrentlyVersing`)
    (bind _output_get (set `self.CurrentVersingTimer` (+ (`self.CurrentVersingTimer`) DeltaSeconds)))
    (bind _returnvalue (/ _output_get (`self.VersingDuration`)))
    (`self.UpdateLiquidHeight` (`KismetMathLibrary.Lerp` (`self.StartingA`) (`self.TargetA`) _returnvalue) (`KismetMathLibrary.Lerp` (`self.StartingB`) (`self.TargetB`) _returnvalue) (`KismetMathLibrary.Lerp` (`self.StartingC`) (`self.TargetC`) _returnvalue))
    (if (>= (`self.CurrentVersingTimer`) (`self.VersingDuration`))
      (set `self.CurrentlyVersing` false)
      (`self.UpdateLiquidHeight` (`self.TargetA`) (`self.TargetB`) (`self.TargetC`)))))

(fn `SetStartingBottleHeight`
  (params (BottleA :type "Float (double-precision)") (BottleB :type "Float (double-precision)") (BottleC :type "Float (double-precision)"))
  (bind _bottle_a (`self.Bottle_A`))
  (bind _bottle_b (`self.Bottle_B`))
  (bind _bottle_c (`self.Bottle_C`))
  (bind (_relativescale3d_x _relativescale3d_y) (`KismetMathLibrary.BreakVector` (`SceneComponent.RelativeScale3D` _bottle_c)))
  (bind (_relativescale3d_x_2 _relativescale3d_y_2) (`KismetMathLibrary.BreakVector` (`SceneComponent.RelativeScale3D` _bottle_a)))
  (bind (_relativescale3d_x_3 _relativescale3d_y_3) (`KismetMathLibrary.BreakVector` (`SceneComponent.RelativeScale3D` _bottle_b)))
  (`SceneComponent.SetRelativeScale3D` _bottle_a (`KismetMathLibrary.MakeVector` _relativescale3d_x_2 _relativescale3d_y_2 BottleA))
  (`SceneComponent.SetRelativeScale3D` _bottle_b (`KismetMathLibrary.MakeVector` _relativescale3d_x_3 _relativescale3d_y_3 BottleB))
  (`SceneComponent.SetRelativeScale3D` _bottle_c (`KismetMathLibrary.MakeVector` _relativescale3d_x _relativescale3d_y BottleC)))

(fn `StartTransferVisually`
  (params (StartA :type "Float (double-precision)") (TargetA :type "Float (double-precision)") (StartB :type "Float (double-precision)") (TargetB :type "Float (double-precision)") (StartC :type "Float (double-precision)") (TargetC :type "Float (double-precision)"))
  (bind _targetb (`self.TargetB`))
  (set `self.CurrentVersingTimer` 0.0)
  (set `self.CurrentlyVersing` true)
  (set `self.StartingA` StartA)
  (set `self.TargetA` TargetA)
  (set `self.StartingB` StartB)
  (set `self.TargetB` TargetB)
  (set `self.StartingC` StartC)
  (set `self.TargetC` TargetC)
  (if (and (`KismetMathLibrary.InRange_FloatFloat` (`self.TargetA`) (- _targetb 0.05) (+ _targetb 0.05)) (== _targetb 0.4))
    (`/Game/Programming/Blueprints/GPE/NewBottlepuzzle/BP_WTP_Manager.Puzzle Finished` (`self.Manager ref`))))

(fn `UpdateLiquidHeight`
  (params (LiquidA_Height :type "Float (double-precision)") (LiquidB_Height :type "Float (double-precision)") (LiquidC_Height :type "Float (double-precision)"))
  (bind _liquid_a (`self.Liquid_A`))
  (bind _liquid_b (`self.Liquid_B`))
  (bind _liquid_c (`self.Liquid_C`))
  (bind (_relativescale3d_x _relativescale3d_y) (`KismetMathLibrary.BreakVector` (`SceneComponent.RelativeScale3D` _liquid_c)))
  (bind (_relativescale3d_x_2 _relativescale3d_y_2) (`KismetMathLibrary.BreakVector` (`SceneComponent.RelativeScale3D` _liquid_a)))
  (bind (_relativescale3d_x_3 _relativescale3d_y_3) (`KismetMathLibrary.BreakVector` (`SceneComponent.RelativeScale3D` _liquid_b)))
  (`SceneComponent.SetRelativeScale3D` _liquid_a (`KismetMathLibrary.MakeVector` _relativescale3d_x_2 _relativescale3d_y_2 LiquidA_Height))
  (`SceneComponent.SetRelativeScale3D` _liquid_b (`KismetMathLibrary.MakeVector` _relativescale3d_x_3 _relativescale3d_y_3 LiquidB_Height))
  (`SceneComponent.SetRelativeScale3D` _liquid_c (`KismetMathLibrary.MakeVector` _relativescale3d_x _relativescale3d_y LiquidC_Height)))

(fn `UserConstructionScript`)