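; Manager actor for a light puzzle that tracks whether every puzzle light is activated.
; On BeginPlay it gathers all BP_LightPuzzle_Light actors in the level into a Lights array.
; CheckVictory scans that array, stops at the first inactive light, and only prints a victory message when all are activated.
; Nothing in this Blueprint calls CheckVictory itself.
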(event `self.ReceiveBeginPlay`
  (bind _outactors (`GameplayStatics.GetAllActorsOfClass` "/Game/Programming/Blueprints/GPE/BP_LightPuzzle_Light.BP_LightPuzzle_Light_C"))
  (set `self.Lights` _outactors))

(fn `CheckVictory`
  (locals (all_activated :type Boolean))
  (set `local.all_activated` true)
  (for _array_element (`self.Lights`)
    (if (not (`/Game/Programming/Blueprints/GPE/BP_LightPuzzle_Light.Activated` _array_element))
      (set `local.all_activated` false)
      (break)))
  (if (`local.all_activated`)
    (`KismetSystemLibrary.PrintString` "gégé" true true (struct :`G` 0.578125 :`B` 0.112094 :`A` 1.0))))

(fn `UserConstructionScript`)