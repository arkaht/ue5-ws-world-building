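; BP_ColorSequence_Input is an interactable button that feeds one color into a color sequence GPE run by an assigned Sequencer.
; On BeginPlay it registers itself with the Sequencer, or prints a warning if none is assigned.
; Interaction through its interaction component sends its ColorID to the Sequencer and prints the returned result.
; A SetColorMaterial function sets the button mesh's material.
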(event `self.ReceiveBeginPlay`
  ;[1 1 1 0.33] Register Input
  (bind _sequencer (`self.Sequencer`)
    (:`then`
      (`/Game/Programming/Blueprints/GPE/BP_ColorSequencer.Register Input` _sequencer self))
    (:`else`
      (`KismetSystemLibrary.PrintString` "BP_ColorSequence_Input: no Sequencer has been assigned, the Input won't work as intended" true true (struct :`R` 1.0 :`G` 0.083333 :`A` 1.0) 10.0))))

(event `self.BP_InteractionComponent.On Interact`
  (params (`Player Controller` :type "/Game/Programming/Blueprints/Core/BP_PlayerController Object Reference"))
  (bind _is_correct (`/Game/Programming/Blueprints/GPE/BP_ColorSequencer.Add Sequence Input` (`self.Sequencer`) (`self.Color ID`)))
  (`KismetSystemLibrary.PrintString` (`KismetStringLibrary.Conv_BoolToString` _is_correct)))

(fn `Set Color Material`
  (params (Material :type "MaterialInterface Object Reference"))
  (`PrimitiveComponent.SetMaterial` (`self.SM Button`) 0 Material))

(fn `UserConstructionScript`)