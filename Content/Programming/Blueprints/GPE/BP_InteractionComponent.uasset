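; Actor component that makes its owner interactable by players, with a cooldown between uses.
; On BeginPlay it finds the owner's "Trigger"-tagged shape, whose overlaps register or unregister it with the BP_PlayerController, and collects "Interaction Outline"-tagged meshes.
; Interact restarts the use timer that Tick counts down, and CanInteract checks that timer plus an optional BPI_Interactable callback on the owner.
; Selection toggles custom depth rendering on the outline meshes.
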(event `self.ReceiveBeginPlay`
  (bind _use_time (`self.Use Time`))
  ;[1 1 1 0.33] Set Use Time
  (set `self.Use Time` (`KismetMathLibrary.SelectFloat` (`/Game/Programming/Blueprints/Data/BP_PlayerData.Interaction Use Time` (`self.Player Data`)) _use_time (== _use_time -1.0)))
  (`self.Find Trigger Collision`)
  (`self.Find Outline Meshes`))

(event `self.ReceiveTick`
  (params (DeltaSeconds :type "Float (single-precision)"))
  (bind _current_use_time (`self.Current Use Time`))
  ;[1 1 1 0.33] Decrease Use Time
  (if (> _current_use_time 0.0)
    (bind _output_get (set `self.Current Use Time` (- _current_use_time DeltaSeconds)))
    (if (<= _output_get 0.0)
      (`self.On Use Time Ready`))))

(event `On Trigger Begin Overlap`
  (params (OverlappedComponent :type "PrimitiveComponent Object Reference") (OtherActor :type "Actor Object Reference") (OtherComp :type "PrimitiveComponent Object Reference") (OtherBodyIndex :type Integer) (bFromSweep :type Boolean) (SweepResult :type "HitResult Structure (by ref)"))
  ;[1 1 1 0.33] Player Trigger
  (bind _asbp_player (cast `/Game/Programming/Blueprints/Core/BP_Player` OtherActor))
  (bind _asbp_player_controller (cast `/Game/Programming/Blueprints/Core/BP_PlayerController` (`Pawn.GetController` _asbp_player)))
  (`/Game/Programming/Blueprints/Core/BP_PlayerController.Add Interaction` _asbp_player_controller self))

(event `On Tigger End Overlap`
  (params (OverlappedComponent :type "PrimitiveComponent Object Reference") (OtherActor :type "Actor Object Reference") (OtherComp :type "PrimitiveComponent Object Reference") (OtherBodyIndex :type Integer))
  ;[1 1 1 0.33] Player Trigger
  (bind _asbp_player (cast `/Game/Programming/Blueprints/Core/BP_Player` OtherActor))
  (bind _asbp_player_controller (cast `/Game/Programming/Blueprints/Core/BP_PlayerController` (`Pawn.GetController` _asbp_player)))
  (`/Game/Programming/Blueprints/Core/BP_PlayerController.Remove Interaction` _asbp_player_controller self))

(fn `Can Interact`
  (params (`Player Controller` :type "/Game/Programming/Blueprints/Core/BP_PlayerController Object Reference"))
  (returns (`Can Interact` :type Boolean))
  (bind _returnvalue (`self.GetOwner`))
  (if (<= (`self.Current Use Time`) 0.0)
    ;[1 1 1 0.33] Custom Callback w/ Interface
    (if (`KismetSystemLibrary.DoesImplementInterface` _returnvalue "/Game/Programming/Blueprints/GPE/BPI_Interactable.BPI_Interactable_C")
      (bind _can_interact (message `/Game/Programming/Blueprints/GPE/BPI_Interactable.Can Interact` _returnvalue `Player Controller`))
      (return _can_interact)
      (else
        (return true)))
    (else
      (return false))))

(fn `Find Outline Meshes`
  (bind _outline_meshes (`self.Outline Meshes`))
  (`KismetArrayLibrary.Array_Clear` _outline_meshes)
  (for _array_element (`Actor.GetComponentsByTag` (`self.GetOwner`) "/Script/Engine.MeshComponent" "Interaction Outline")
    (`PrimitiveComponent.SetCustomDepthStencilValue` _array_element 1)
    (`KismetArrayLibrary.Array_Add` _outline_meshes _array_element)))

(fn `Find Trigger Collision`
  (bind _returnvalue (`self.GetOwner`))
  (for _array_element (`Actor.GetComponentsByTag` _returnvalue "/Script/Engine.ShapeComponent" "Trigger")
    (`self.Set Trigger Collision` _array_element)
    (break))
  (`self.Trigger Collision`
    (:`then`)
    (:`else`
      (`KismetSystemLibrary.PrintText` (`|FormatText` "BP_InteractionComponent: the Trigger Collision was not found on {Actor}, be sure to have a Shape Component with the tag 'Trigger' on it" _returnvalue) true true (struct :`R` 1.0 :`G` 0.083333 :`A` 1.0) 10.0))))

(fn `Interact`
  (params (`Player Controller` :type "/Game/Programming/Blueprints/Core/BP_PlayerController Object Reference"))
  ;[1 1 1 0.33] Reset Use Time
  (set `self.Current Use Time` (`self.Use Time`))
  (`self.On Interact` `Player Controller`))

(fn `Set Outline Meshes Render Custom Depth`
  (params (`Is Visible` :type Boolean))
  (for _array_element (`self.Outline Meshes`)
    (`PrimitiveComponent.SetRenderCustomDepth` _array_element `Is Visible`)))

(fn `Set Selected`
  (params (`Is Selected` :type Boolean))
  (bind _output_get (set `self.Is Selected` `Is Selected`))
  (`self.Set Outline Meshes Render Custom Depth` _output_get))

(fn `Set Trigger Collision`
  (params (`Shape Component` :type "ShapeComponent Object Reference"))
  (bind _output_get (set `self.Trigger Collision` `Shape Component`))
  (add `PrimitiveComponent.OnComponentBeginOverlap` _output_get (`|CreateDelegate` :!event `On Trigger Begin Overlap`))
  (add `PrimitiveComponent.OnComponentEndOverlap` _output_get (`|CreateDelegate` :!event `On Tigger End Overlap`)))