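; BP_GardenPlantSpawner is a garden plant object that gets a random appearance when play begins.
; On BeginPlay it picks a random index into MeshList and applies that same mesh to both InteractableMesh and MirroredMesh, so the two always match.
; The construction script is empty, so the random choice happens only at runtime.
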(event `self.ReceiveBeginPlay`
  (bind _output_get (set `self.randomInt` (`KismetMathLibrary.RandomIntegerInRange` 0 (- (`KismetArrayLibrary.Array_Length` (`self.MeshList`)) 1))))
  (bind _output (`|GetArrayItem` (`self.MeshList`) _output_get))
  (`StaticMeshComponent.SetStaticMesh` (`self.InteractableMesh`) _output)
  (`StaticMeshComponent.SetStaticMesh` (`self.MirroredMesh`) _output))

(fn `UserConstructionScript`)