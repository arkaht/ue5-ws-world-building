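; Gargantua-style black hole prop whose look is tuned through exposed variables on the actor.
; The construction script pushes those variables into material parameters on two components: Blackhole for size, event horizon, accretion disk color, Doppler, emission, ring and quality steps, and OuterLensing for fresnel and refraction.
; All visuals come from the materials; the event graph has no active runtime logic.
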(fn `UserConstructionScript`
  (bind _blackhole (`self.Blackhole`))
  (bind _outer_lensing (`self.Outer_Lensing`))
  (`MeshComponent.SetScalarParameterValueOnMaterials` _blackhole "Blackhole_Size" (`self.Blackhole Size`))
  (`MeshComponent.SetVectorParameterValueOnMaterials` _blackhole "Accreation_Disk_Color" (`self.Accreation Disk Color`))
  (`MeshComponent.SetScalarParameterValueOnMaterials` _blackhole "Quality_Steps" (`self.Quality Steps`))
  (`MeshComponent.SetScalarParameterValueOnMaterials` _blackhole "Doppler_Intensity" (`self.Doppler Intensity`))
  (`MeshComponent.SetScalarParameterValueOnMaterials` _blackhole "Event_Horizon_Size" (`self.Event Horizon Size`))
  (`MeshComponent.SetScalarParameterValueOnMaterials` _blackhole "Emission_Intensity" (`self.Emission Intensity`))
  (`MeshComponent.SetScalarParameterValueOnMaterials` _blackhole "Ring_Radius" (`self.Ring_Radius`))
  (`MeshComponent.SetScalarParameterValueOnMaterials` _blackhole "Rotation_Ring_Speed" (`self.Rotation_Ring_Speed`))
  (`MeshComponent.SetScalarParameterValueOnMaterials` _blackhole "Ring_Intensity" (`self.Ring Intensity`))
  (`MeshComponent.SetScalarParameterValueOnMaterials` _blackhole "Ring_Intensity_Falloff" (`self.Ring Intensity Falloff`))
  (`MeshComponent.SetScalarParameterValueOnMaterials` _blackhole "iring" (`self.I Ring`))
  (`MeshComponent.SetScalarParameterValueOnMaterials` _outer_lensing "Fresnel_Intensity" (`self.Fresnel Intensity`))
  (`MeshComponent.SetScalarParameterValueOnMaterials` _outer_lensing "Refraction_Power" (`self.Refraction Power`)))