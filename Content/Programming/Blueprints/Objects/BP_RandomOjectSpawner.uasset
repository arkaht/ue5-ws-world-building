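; Spawner actor that places seven distinct, randomly chosen pickable objects (trophies) across rooms when play begins.
; BeginPlay gathers all BP_ObjectSpawnPoint actors and rerolls random item indices against an already-spawned array to avoid duplicates.
; SpawnTrophy then spawns one object per room index at the first matching spawn point and sets its E_PickableObject type.
; Older random spawn-point selection logic remains in the graph but never runs.
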(event `self.ReceiveBeginPlay`
  ;[1 1 1] Get all spawn point
  (bind _outactors (`GameplayStatics.GetAllActorsOfClass` "/Game/Programming/Blueprints/Objects/BP_ObjectSpawnPoint.BP_ObjectSpawnPoint_C"))
  (set `self.SpawnPoints` _outactors)
  (while (!= (`self.spawnedItemCount`) 7)
    ;[1 1 1] Loop to select an item
    (while (not (`self.ObjectFound`))
      ;[1 1 1] Get a random item and check if this item is already spawned
      (bind _output_get (set `self.itemToSpawnIndex` (`KismetMathLibrary.RandomIntegerInRange` 0 15) :!label _label))
      (if (== (`|GetArrayItem` (`self.AlreadySpawned`) _output_get) false)
        ;[1 1 1] Change item count and set item as spawned
        (`KismetArrayLibrary.Array_Set` (`self.SelectedActors`) (`self.spawnedItemCount`) (`self.itemToSpawnIndex`))
        (set `self.spawnedItemCount` (+ (`self.spawnedItemCount`) 1))
        (`KismetArrayLibrary.Array_Set` (`self.AlreadySpawned`) (`self.itemToSpawnIndex`) true)
        (set `self.ObjectFound` true)
        (else
          (goto _label))))
    (set `self.ObjectFound` false))
  (for _index (range 7)
    (`self.Spawn Trophy` _index)))

(fn `Spawn Trophy`
  (params (RoomIndex :type Integer))
  (for (_array_element _array_index) (`self.SpawnPoints`)
    (if (== (`/Game/Programming/Blueprints/Objects/BP_ObjectSpawnPoint.RoomIndex` _array_element) RoomIndex)
      (`|ExecutionSequence`
        (:`then_0`
          ;[1 1 1] Spawn actor
          (bind _returnvalue (`|SpawnActorFromClass` (`self.Object`) (`self.GetTransform` (`|GetArrayItem` (`self.SpawnPoints`) _array_index)) "Undefined" "OverrideRootScale" null null))
          (`/Game/Programming/Blueprints/Objects/BP_Object.SetObject` _returnvalue (cast `/Game/Programming/Enums/E_PickableObject` (`KismetMathLibrary.Conv_IntToByte` (`|GetArrayItem` (`self.SelectedActors`) RoomIndex)))))
        (:`then_1`
          (break))))))

(fn `UserConstructionScript`)