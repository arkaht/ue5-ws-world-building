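; BP_RulesTrigger is a trigger actor that shows a room's rules in the game mode's in-game menu.
; On player overlap, for one Room value (the potion maker), it appends the cauldron's target color to the rules text and caches the menu.
; It then either toggles a press-key prompt or shows the rules once automatically.
; The R key also shows them while the player is inside, and prints debug text.
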(event `Key|R` :consume false
  (params (Key :type "Key Structure"))
  (:`Pressed`
    (`KismetSystemLibrary.PrintString` (`KismetStringLibrary.Conv_BoolToString` (`self.CanOpenRule`)))))

(event `self.ReceiveBeginPlay`
  (`self.EnableInput` (`GameplayStatics.GetPlayerController` 0)))

(event `self.ReceiveActorBeginOverlap`
  (params (OtherActor :type "Actor Object Reference"))
  (cast `/Game/Programming/Blueprints/Core/BP_Player` OtherActor)
  (set `self.CanOpenRule` true)
  (bind _asbp_gamemode (cast `/Game/Programming/Blueprints/Core/BP_Gamemode` (`GameplayStatics.GetGameMode`)))
  ;[1 1 1] Change Color target for PotionMaker
  (if (`|EnumEquality` (`self.Room`) "NewEnumerator4")
    (bind _ingamemenu (`/Game/Programming/Blueprints/Core/BP_Gamemode.InGameMenu` _asbp_gamemode))
    (bind _gametexts (`/Game/Programming/Blueprints/UI/BP_InGame.GameTexts` _ingamemenu))
    (`KismetArrayLibrary.Array_Set` _gametexts 4 (`|FormatText` "{initText} \nTarget Color: {targetColor}" (`|GetArrayItem` _gametexts 4) (`|GetEnumeratorNameAsString` (`/Game/Programming/Blueprints/GPE/BP_PotionMaker.ColorResult` (`self.GPE_Chaudron`)))))
    (set `self.In Game Menu` _ingamemenu)
    (if (`self.PressKeyToOpenRules`)
      (`/Game/Programming/Blueprints/UI/BP_InGame.SetShowPressKeyRules` (`self.In Game Menu`) true)
      (elif (not (`self.alreadyShowed`))
        (set `self.alreadyShowed` true)
        (if (`self.CanOpenRule`) :!label _label
          (`KismetSystemLibrary.PrintString` "Hello")
          (`/Game/Programming/Blueprints/UI/BP_InGame.Show Rules` (`self.In Game Menu`) (`self.Room`)))))))

(event `Key|R` :consume false
  (params (Key :type "Key Structure"))
  (:`Pressed`
    (goto _label)))

(event `self.ReceiveActorEndOverlap`
  (params (OtherActor :type "Actor Object Reference"))
  (cast `/Game/Programming/Blueprints/Core/BP_Player` OtherActor)
  (set `self.CanOpenRule` false)
  (if (`self.PressKeyToOpenRules`)
    (`/Game/Programming/Blueprints/UI/BP_InGame.SetShowPressKeyRules` (`self.In Game Menu`) false)))

(fn `UserConstructionScript`)