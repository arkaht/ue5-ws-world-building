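; BP_Object is an actor that can appear as one of sixteen assorted props, such as a radish, trumpet or bowling ball.
; SetObject switches on the ItemToShow value and makes the matching numbered component visible, without propagating to children.
; It never hides the other components, and the event graph and construction script are empty, so display depends on an external call.
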(fn `SetObject`
  (params (ItemToShow :type "/Game/Programming/Enums/E_PickableObject Enum" :default "NewEnumerator0"))
  (switch `/Game/Programming/Enums/E_PickableObject` ItemToShow
    (:`NewEnumerator0`
      (`SceneComponent.SetVisibility` (`self.Object0`) true false))
    (:`NewEnumerator1`
      (`SceneComponent.SetVisibility` (`self.Object1`) true false))
    (:`NewEnumerator2`
      (`SceneComponent.SetVisibility` (`self.Object2`) true false))
    (:`NewEnumerator3`
      (`SceneComponent.SetVisibility` (`self.Object3`) true false))
    (:`NewEnumerator4`
      (`SceneComponent.SetVisibility` (`self.Object4`) true false))
    (:`NewEnumerator5`
      (`SceneComponent.SetVisibility` (`self.Object5`) true false))
    (:`NewEnumerator6`
      (`SceneComponent.SetVisibility` (`self.Object6`) true false))
    (:`NewEnumerator7`
      (`SceneComponent.SetVisibility` (`self.Object7`) true false))
    (:`NewEnumerator8`
      (`SceneComponent.SetVisibility` (`self.Object8`) true false))
    (:`NewEnumerator9`
      (`SceneComponent.SetVisibility` (`self.Object9`) true false))
    (:`NewEnumerator10`
      (`SceneComponent.SetVisibility` (`self.Object10`) true false))
    (:`NewEnumerator11`
      (`SceneComponent.SetVisibility` (`self.Object11`) true false))
    (:`NewEnumerator12`
      (`SceneComponent.SetVisibility` (`self.Object12`) true false))
    (:`NewEnumerator13`
      (`SceneComponent.SetVisibility` (`self.Object13`) true false))
    (:`NewEnumerator14`
      (`SceneComponent.SetVisibility` (`self.Object14`) true false))
    (:`NewEnumerator15`
      (`SceneComponent.SetVisibility` (`self.Object15`) true false))))

(fn `UserConstructionScript`)