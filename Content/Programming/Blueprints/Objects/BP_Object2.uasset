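; Interactable trophy object that can appear as one of sixteen props, such as a pizza, trumpet or bowling ball.
; SetObject hides all variants, shows the one matching the item type and caches its first child mesh.
; Tick raises the actor from 400 units below its starting height over one second after spawning.
; Interacting while the player holds nothing disables the box's overlap events and passes the object to BP_Player's OnTrophyInteraction.
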(event `self.ReceiveBeginPlay`
  (set `self.StartZPos` (.z (`self.K2_GetActorLocation`))))

(event `self.BP_InteractionComponent.On Interact`
  (params (`Player Controller` :type "/Game/Programming/Blueprints/Core/BP_PlayerController Object Reference"))
  (bind _bp_player (`/Game/Programming/Blueprints/Core/BP_PlayerController.BP Player` `Player Controller`))
  (`KismetSystemLibrary.PrintString` "Hello")
  (if (not (`/Game/Programming/Blueprints/Core/BP_Player.IsGrabbingObject?` _bp_player))
    (set `PrimitiveComponent.bGenerateOverlapEvents` false (`self.Box`))
    (`/Game/Programming/Blueprints/Core/BP_Player.OnTrophyInteraction` _bp_player self)))

(event `self.ReceiveTick`
  (params (DeltaSeconds :type "Float (single-precision)"))
  (if (< (`self.AnimationTimer`) 1.0)
    (set `self.AnimationTimer` (+ (`self.AnimationTimer`) DeltaSeconds))
    (`self.K2_SetActorLocation` (`KismetMathLibrary.MakeVector` (.x (`self.K2_GetActorLocation`)) (.y (`self.K2_GetActorLocation`)) (- (`self.StartZPos`) (* (- 1.0 (`self.AnimationTimer`)) 400.0))))
    (else
      (set `self.AnimationTimer` 1.0))))

(event `self.BP_InteractionComponent.OnComponentActivated`
  (params (Component :type "ActorComponent Object Reference") (bReset :type Boolean))
  (`KismetSystemLibrary.PrintString` (`KismetSystemLibrary.GetDisplayName` Component)))

(fn `Can Interact`
  (params (`Player Controller` :type "/Game/Programming/Blueprints/Core/BP_PlayerController Object Reference"))
  (returns (`Can Interact` :type Boolean))
  (return true))

(fn `Set Mesh`
  (params (Scene :type "SceneComponent Object Reference"))
  (bind _asmesh_component (cast `MeshComponent` (`SceneComponent.GetChildComponent` Scene 0)))
  (set `self.Mesh` _asmesh_component))

(fn `SetObject`
  (params (ItemToShow :type "/Game/Programming/Enums/E_PickableObject Enum" :default "NewEnumerator0"))
  (bind _object0 (`self.Object0`))
  (bind _object1 (`self.Object1`))
  (bind _object2 (`self.Object2`))
  (bind _object3 (`self.Object3`))
  (bind _object4 (`self.Object4`))
  (bind _object5 (`self.Object5`))
  (bind _object6 (`self.Object6`))
  (bind _object7 (`self.Object7`))
  (bind _object8 (`self.Object8`))
  (bind _object9 (`self.Object9`))
  (bind _object10 (`self.Object10`))
  (bind _object11 (`self.Object11`))
  (bind _object12 (`self.Object12`))
  (bind _object13 (`self.Object13`))
  (bind _object14 (`self.Object14`))
  (bind _object15 (`self.Object15`))
  (`SceneComponent.SetVisibility` (`self.Object0`) false true)
  (`SceneComponent.SetVisibility` (`self.Object1`) false true)
  (`SceneComponent.SetVisibility` (`self.Object2`) false true)
  (`SceneComponent.SetVisibility` (`self.Object3`) false true)
  (`SceneComponent.SetVisibility` (`self.Object4`) false true)
  (`SceneComponent.SetVisibility` (`self.Object5`) false true)
  (`SceneComponent.SetVisibility` (`self.Object6`) false true)
  (`SceneComponent.SetVisibility` (`self.Object7`) false true)
  (`SceneComponent.SetVisibility` (`self.Object8`) false true)
  (`SceneComponent.SetVisibility` (`self.Object10`) false true)
  (`SceneComponent.SetVisibility` (`self.Object11`) false true)
  (`SceneComponent.SetVisibility` (`self.Object12`) false true)
  (`SceneComponent.SetVisibility` (`self.Object13`) false true)
  (`SceneComponent.SetVisibility` (`self.Object14`) false true)
  (`SceneComponent.SetVisibility` (`self.Object15`) false true)
  (`SceneComponent.SetVisibility` (`self.Object9`) false true)
  (bind _output_get (set `self.ItemType` ItemToShow))
  (switch `/Game/Programming/Enums/E_PickableObject` _output_get
    (:`NewEnumerator0`
      (`SceneComponent.SetVisibility` _object0 true true)
      (`self.Set Mesh` _object0))
    (:`NewEnumerator1`
      (`SceneComponent.SetVisibility` _object1 true true)
      (`self.Set Mesh` _object1))
    (:`NewEnumerator2`
      (`SceneComponent.SetVisibility` _object2 true true)
      (`self.Set Mesh` _object2))
    (:`NewEnumerator3`
      (`SceneComponent.SetVisibility` _object3 true true)
      (`self.Set Mesh` _object3))
    (:`NewEnumerator4`
      (`SceneComponent.SetVisibility` _object4 true true)
      (`self.Set Mesh` _object4))
    (:`NewEnumerator5`
      (`SceneComponent.SetVisibility` _object5 true true)
      (`self.Set Mesh` _object5))
    (:`NewEnumerator6`
      (`SceneComponent.SetVisibility` _object6 true true)
      (`self.Set Mesh` _object6))
    (:`NewEnumerator7`
      (`SceneComponent.SetVisibility` _object7 true true)
      (`self.Set Mesh` _object7))
    (:`NewEnumerator8`
      (`SceneComponent.SetVisibility` _object8 true true)
      (`self.Set Mesh` _object8))
    (:`NewEnumerator9`
      (`SceneComponent.SetVisibility` _object9 true true)
      (`self.Set Mesh` _object9))
    (:`NewEnumerator10`
      (`SceneComponent.SetVisibility` _object10 true true)
      (`self.Set Mesh` _object10))
    (:`NewEnumerator11`
      (`SceneComponent.SetVisibility` _object11 true true)
      (`self.Set Mesh` _object11))
    (:`NewEnumerator12`
      (`SceneComponent.SetVisibility` _object12 true true)
      (`self.Set Mesh` _object12))
    (:`NewEnumerator13`
      (`SceneComponent.SetVisibility` _object13 true true)
      (`self.Set Mesh` _object13))
    (:`NewEnumerator14`
      (`SceneComponent.SetVisibility` _object14 true true)
      (`self.Set Mesh` _object14))
    (:`NewEnumerator15`
      (`SceneComponent.SetVisibility` _object15 true true)
      (`self.Set Mesh` _object15))))

(fn `UserConstructionScript`)