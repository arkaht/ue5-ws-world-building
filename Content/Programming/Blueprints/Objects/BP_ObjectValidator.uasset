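; BP_ObjectValidator is an interactable drop-off point where the player deposits trophies to progress toward winning.
; On interact while grabbing, it takes the held actor from BP_Player and snaps it to TrophyPosition.
; Tick then drives a dither fade on the mesh until a timer destroys the actor.
; Each destruction updates the in-game menu's trophy count and prints a game-over message at the target count.
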(event `self.ReceiveBeginPlay`)

(event `self.ReceiveTick`
  (params (DeltaSeconds :type "Float (single-precision)"))
  (if (`KismetSystemLibrary.IsValid` (`self.Actor to Pick`))
    (bind _output_get (set `self.destroyTimer` (- (`self.destroyTimer`) DeltaSeconds)))
    (if (<= _output_get 0.0)
      (set `self.destroyTimer` 1.0)
      (`self.K2_DestroyActor` (stale `self.BP_InteractionComponent.On Interact` _output_get))
      (bind _output_get_2 (set `self.CollectedTrophyCount` (+ (`self.CollectedTrophyCount`) 1)))
      (bind _asbp_gamemode (cast `/Game/Programming/Blueprints/Core/BP_Gamemode` (`GameplayStatics.GetGameMode`)))
      (`/Game/Programming/Blueprints/UI/BP_InGame.SetTrophyCount` (`/Game/Programming/Blueprints/Core/BP_Gamemode.InGameMenu` _asbp_gamemode) (`self.CollectedTrophyCount`))
      (if (== _output_get_2 (`self.TrophyCountToWin`))
        (`KismetSystemLibrary.PrintString` "JEU FINI"))
      (else
        (bind _asbp_object (cast `/Game/Programming/Blueprints/Objects/BP_Object` (`self.Actor to Pick`)))
        (`MeshComponent.SetScalarParameterValueOnMaterials` (`/Game/Programming/Blueprints/Objects/BP_Object.Mesh` _asbp_object) "DitherAmount" (- 1.0 _output_get))))))

(event `self.BP_InteractionComponent.On Interact`
  (params (`Player Controller` :type "/Game/Programming/Blueprints/Core/BP_PlayerController Object Reference"))
  (bind _bp_player (`/Game/Programming/Blueprints/Core/BP_PlayerController.BP Player` `Player Controller`))
  (`KismetSystemLibrary.PrintString` "Hello")
  (if (`/Game/Programming/Blueprints/Core/BP_Player.IsGrabbingObject?` _bp_player)
    (set `/Game/Programming/Blueprints/Core/BP_Player.CanDropHoldingObject?` true _bp_player)
    (`KismetSystemLibrary.PrintString` "Tentative de posage de Trophé")
    (bind _returnvalue (`GameplayStatics.GetActorOfClass` "/Game/Programming/Blueprints/Core/BP_Player.BP_Player_C"))
    (bind _output_get (set `self.Actor to Pick` (`/Game/Programming/Blueprints/Core/BP_Player.ActorToPick` _returnvalue)))
    (`/Game/Programming/Blueprints/Core/BP_Player.OnTrophyInteraction` _returnvalue _output_get)
    (`self.K2_SetActorLocation` _output_get (`SceneComponent.K2_GetComponentLocation` (`self.TrophyPosition`)) false false)))

(fn `UserConstructionScript`)