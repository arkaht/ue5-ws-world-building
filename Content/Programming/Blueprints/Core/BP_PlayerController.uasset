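; Player controller Blueprint that routes the Interact input to whatever interaction the player pawn currently holds.
; On BeginPlay it caches the controlled pawn as BP_Player, printing an on-screen error if the cast fails.
; On Interact press it validates the pawn's CurrentInteraction, asks it CanInteract, then calls Interact, passing itself as the controller to both calls.
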(event `self.ReceiveBeginPlay`
  ;[1 1 1 0.33] Retrieve BP Player
  (bind _asbp_player (cast `/Game/Programming/Blueprints/Core/BP_Player` (`self.K2_GetPawn`))
    (:`then`
      (set `self.BP Player` _asbp_player))
    (:`CastFailed`
      (`KismetSystemLibrary.PrintString` "BP_PlayerController: failed to retrieve BP_Player" true true (struct :`R` 1.0 :`G` 0.083333 :`A` 1.0) 5.0))))

(event `InputAction|Interact`
  (params (Key :type "Key Structure"))
  ;[1 1 1 0.33] Interaction
  (:`Pressed`
    (bind _current_interaction (`/Game/Programming/Blueprints/Core/BP_Player.Current Interaction` (`self.BP Player`))
      (:`then`
        (bind _can_interact (`/Game/Programming/Blueprints/GPE/BP_InteractionComponent.Can Interact` _current_interaction self))
        (if _can_interact
          (`/Game/Programming/Blueprints/GPE/BP_InteractionComponent.Interact` _current_interaction self)))
      (:`else`))))

(fn `UserConstructionScript`)