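; Machine room manager that switches the room to its powered, unlocked state when BP_ColorSequencer spawns the trophy.
; BeginPlay gathers the pistons, meters and object stand, then caches each tank's emissive material and blacks it out.
; On trophy spawn, one sequence recolors the mood light, stops sparks, starts pistons, normalizes meters, restores tank materials, enables arcs, arc lights, stand light and pipe smoke, and unlocks the door.
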(event `self.BP_ColorSequencer.On Trophy Spawn`
  (bind _lightcomponent (`Light.LightComponent` (`self.MoodRectLight`)))
  (`|ExecutionSequence`
    (:`then_0`
      (`LightComponent.SetLightColor` _lightcomponent (struct :`R` 0.360784 :`G` 0.643137 :`B` 0.8 :`A` 1.0) true)
      (`LightComponent.SetVolumetricScatteringIntensity` _lightcomponent 2.0)
      (`LightComponent.SetIntensity` _lightcomponent 30.0))
    (:`then_1`
      (for _array_element (`self.SparksFX`)
        (`FXSystemComponent.SetFloatParameter` (`NiagaraActor.NiagaraComponent` _array_element) "Spawn Rate" 0.0)
        (`KismetSystemLibrary.Delay` 1.0)
        (`self.K2_DestroyActor` _array_element)))
    (:`then_2`
      (for _array_element_2 (`self.Piston`)
        (`/Game/Art/Meshes/5_MACHINEROOM/1_Props/SM_P_Dinner_Piston_Animated.EnablePistonAnimation` _array_element_2)))
    (:`then_3`
      (for _array_element_3 (`self.MachineRoomMeterAligned`)
        (`/Game/Art/Meshes/5_MACHINEROOM/1_Props/SM_P_MachineRoom_Meter_Animated.ResetRandomToNormal` _array_element_3)))
    (:`then_4`
      (for (_array_element_4 _array_index) (`self.Tank`)
        (`PrimitiveComponent.SetMaterial` (`StaticMeshActor.StaticMeshComponent` _array_element_4) 1 (`|GetArrayItem` (`self.TankEmissiveMat`) _array_index))))
    (:`then_5`
      (for _array_element_5 (`self.ElectricArcs`)
        (`self.SetActorHiddenInGame` _array_element_5 false)))
    (:`then_6`
      (for _array_element_6 (`self.ElecArcsLight`)
        (`LightComponent.SetIntensity` (`Light.LightComponent` _array_element_6) 30.0)))
    (:`then_7`
      (`/Game/Art/Meshes/5_MACHINEROOM/Anim/BP_Object_Stand.TurnOnLight` (`self.BP_ObjectStand`)))
    (:`then_8`
      (for _array_element_7 (`self.NS_PipeSmoke`)
        (`FXSystemComponent.SetFloatParameter` (`NiagaraActor.NiagaraComponent` _array_element_7) "SpawnRate" 100.0)))
    (:`then_9`
      (set `/Game/Programming/Blueprints/Props/BP_Door.IsLocked` false (`self.Door`)))))

(event `self.ReceiveBeginPlay`
  (bind _outactors (`GameplayStatics.GetAllActorsOfClass` "/Game/Art/Meshes/5_MACHINEROOM/1_Props/SM_P_Dinner_Piston_Animated.SM_P_Dinner_Piston_Animated_C"))
  (set `self.Piston` _outactors)
  (bind _outactors_2 (`GameplayStatics.GetAllActorsOfClass` "/Game/Art/Meshes/5_MACHINEROOM/1_Props/SM_P_MachineRoom_Meter_Animated.SM_P_MachineRoom_Meter_Animated_C"))
  (set `self.MachineRoomMeterAligned` _outactors_2)
  (bind _returnvalue (`GameplayStatics.GetActorOfClass` "/Game/Art/Meshes/5_MACHINEROOM/Anim/BP_Object_Stand.BP_Object_Stand_C"))
  (set `self.BP_ObjectStand` _returnvalue)
  (for _array_element (`self.Tank`)
    (bind _staticmeshcomponent (`StaticMeshActor.StaticMeshComponent` _array_element))
    (`KismetArrayLibrary.Array_Add` (`self.TankEmissiveMat`) (`PrimitiveComponent.GetMaterial` _staticmeshcomponent 1))
    (`PrimitiveComponent.SetMaterial` _staticmeshcomponent 1 "/Game/Art/Materials/Instances/FlatColors/I_Black_1.I_Black_1")))

(fn `UserConstructionScript`)